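; Spawner actor that spawns random zombies or bosses from game mode lists while it is not day.
; Tick drives a DoOnce-gated roll against SpawnRate, paced by SpawnDelay, and a box overlap blocks spawning while zombies occupy it.
; SpawnEnemy picks the boss from debug BossMode or game mode SpawnBoss, spawning it only if exactly one of its class exists, otherwise a zombie.
; Spawns get a random Y offset.
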(event OnComponentBeginOverlap(Box)
  (params (OverlappedComponent :type Primitive%20Component%20Object%20Reference) (OtherActor :type Actor%20Object%20Reference) (OtherComp :type Primitive%20Component%20Object%20Reference) (OtherBodyIndex :type Integer) (bFromSweep :type Boolean) (SweepResult :type Hit%20Result%20Structure%20%28by%20ref%29))
  (Utilities|Casting|CastToenemyZombie OtherActor)
  (if true
    (Variables|Default|SetcanSpawn false)))

(event OnComponentEndOverlap(Box)
  (params (OverlappedComponent :type Primitive%20Component%20Object%20Reference) (OtherActor :type Actor%20Object%20Reference) (OtherComp :type Primitive%20Component%20Object%20Reference) (OtherBodyIndex :type Integer))
  (bind _asenemy_zombie (Utilities|Casting|CastToenemyZombie OtherActor))
  (if (< (Utilities|Array|Length (Collision|GetOverlappingActors (Variables|Default|GetBox) (Utilities|GetClass _asenemy_zombie) :!class /Script/Engine.PrimitiveComponent)) 1)
    (Variables|Default|SetcanSpawn true)))

(event EventBeginPlay
  (bind _returnvalue (Actor|GetActorOfClass "/Game/Blueprints/DebugModeBp.DebugModeBp_C"))
  (Variables|Default|SetdebugBp _returnvalue)
  (bind _asfp_sgame_mode_base (Utilities|Casting|CastToFpSGameModeBase (Game|GetGameMode)))
  (Variables|Default|SetgameMode _asfp_sgame_mode_base))

(event Collision|EventActorBeginOverlap
  (params (OtherActor :type Actor%20Object%20Reference)))

(event EventTick
  (params (DeltaSeconds :type Float%20%28single-precision%29))
  (bind _gamemode (Variables|Default|GetgameMode))
  (bind _asfp_sgame_mode_base (Utilities|Casting|CastToFpSGameModeBase (Game|GetGameMode)))
  (if (not (Variables|/Game/Blueprints/FpSGameModeBase.FpSGameModeBase_C|GetDay? _asfp_sgame_mode_base))
    (Utilities|FlowControl|DoOnce false :!label _label
      (:Completed
        (if (> (Math|Random|RandomIntegerinRange 0 100) (Variables|/Game/Blueprints/FpSGameModeBase.FpSGameModeBase_C|GetspawnRate _gamemode))
          (if (Variables|Default|GetcanSpawn)
            (CallFunction|SpawnEnemy)
            (else
              (goto _label Reset))))
        (Utilities|FlowControl|Delay (Variables|/Game/Blueprints/FpSGameModeBase.FpSGameModeBase_C|GetspawnDelay _gamemode))
        (goto _label Reset)))))

(fn ConstructionScript)

(fn SpawnEnemy
  (bind _vectorfield (Variables|Default|GetVectorField))
  (bind _offset (Variables|Default|Getoffset))
  (bind _gamemode (Variables|Default|GetgameMode))
  (bind _debugbp (Variables|Default|GetdebugBp))
  (bind _gamemode_2 (Variables|Default|GetgameMode))
  (bind _returnvalue (Transformation|GetSocketLocation _vectorfield "None"))
  (bind _returnvalue_2 (* -1.0 _offset))
  (bind _zombies (Variables|/Game/Blueprints/FpSGameModeBase.FpSGameModeBase_C|Getzombies _gamemode))
  (bind _returnvalue_3 (Math|Random|RandomFloatinRange _returnvalue_2 _offset))
  (bind _returnvalue_4 (+ (.y _returnvalue) _returnvalue_3))
  (if (Variables|/Game/Blueprints/DebugModeBp.DebugModeBp_C|GetbossMode _debugbp)
    (Variables|Default|SetnumBoss (Variables|/Game/Blueprints/DebugModeBp.DebugModeBp_C|Getboss _debugbp))
    (bind _outactors (Actor|GetAllActorsOfClass (Utilities|GetClass (Utilities|Array|Get(acopy) (Variables|/Game/Blueprints/FpSGameModeBase.FpSGameModeBase_C|GetbossActors _gamemode_2) (Variables|Default|GetnumBoss))) :!label _label))
    (if (== (Utilities|Array|Length _outactors) 1)
      (Game|SpawnActorfromClass (Utilities|GetClass (Utilities|Array|Get(acopy) (Variables|/Game/Blueprints/FpSGameModeBase.FpSGameModeBase_C|GetbossActors _gamemode_2) (Variables|Default|GetnumBoss))) (Math|Transform|MakeTransform (Math|Vector|MakeVector (.x _returnvalue) _returnvalue_4 1.5e+02) "0, 0, 0" "1,1,1") "Undefined" 0 0)
      (else
        (Game|SpawnActorfromClass (Utilities|GetClass (Utilities|Array|Get(acopy) _zombies (Math|Random|RandomIntegerinRange 0 (Utilities|Array|Length _zombies)))) (Math|Transform|MakeTransform (Math|Vector|MakeVector (.x _returnvalue) _returnvalue_4 1.5e+02) "0, 0, 0" "1,1,1") "Undefined" 0 0 :!label _label_2)))
    (elif (Variables|/Game/Blueprints/FpSGameModeBase.FpSGameModeBase_C|GetspawnBoss _gamemode_2)
      (Variables|Default|SetnumBoss (Variables|/Game/Blueprints/FpSGameModeBase.FpSGameModeBase_C|GetbossCount _gamemode_2))
      (goto _label)
      (else
        (goto _label_2)))))