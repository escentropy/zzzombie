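; Base building Blueprint for the farming area that lets the player repair it by clicking or tapping its mesh.
; A click checks the equipped inventory item's type, then charges the fix cost through the player controller, skipping the cost when the debug actor has Debug enabled.
; Repairs add the item's value as a percentage of the entity's max health, capped at full.
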(event OnClicked(StaticMesh1)
  (params (TouchedComponent :type Primitive%20Component%20Object%20Reference) (ButtonPressed :type Key%20Structure :default "None"))
  (bind _returnvalue (Actor|GetActorOfClass "/Game/Blueprints/DebugModeBp.DebugModeBp_C"))
  (bind _item (Default|GetEquipedItem (Variables|Default|GetInvSysBp) "NewEnumerator5"))
  (if (Utilities|Enum|Equal(Enum) (.Type (Utilities|Struct|BreaktoolsStr (Variables|/Game/Blueprints/Tools/ToolsMaster.ToolsMaster_C|Getinfo _item))) "NewEnumerator4")
    (if (Variables|/Game/Blueprints/DebugModeBp.DebugModeBp_C|Getdebug? _returnvalue)
      (CallFunction|IncreaseHealth (Math|Conversions|ToFloat(Integer) (.value (Utilities|Struct|BreaktoolsStr (Variables|/Game/Blueprints/Tools/ToolsMaster.ToolsMaster_C|Getinfo _item)))) :!label _label)
      (else
        (bind _hasrsc (Default|RemoveRsc (Variables|Default|GetplCont) (Utilities|Struct|BreakentityStats (Variables|Default|GetentStats))))
        (if _hasrsc
          (goto _label))))))

(event OnInputTouchBegin(StaticMesh1)
  (params (FingerIndex :type ETouchIndex%20Enum :default "Touch1") (TouchedComponent :type Primitive%20Component%20Object%20Reference))
  (bind _returnvalue (Actor|GetActorOfClass "/Game/Blueprints/DebugModeBp.DebugModeBp_C"))
  (bind _item (Default|GetEquipedItem (Variables|Default|GetInvSysBp) "NewEnumerator5"))
  (if (Utilities|Enum|Equal(Enum) (.Type (Utilities|Struct|BreaktoolsStr (Variables|/Game/Blueprints/Tools/ToolsMaster.ToolsMaster_C|Getinfo _item))) "NewEnumerator4")
    (if (Variables|/Game/Blueprints/DebugModeBp.DebugModeBp_C|Getdebug? _returnvalue)
      (CallFunction|IncreaseHealth (Math|Conversions|ToFloat(Integer) (.value (Utilities|Struct|BreaktoolsStr (Variables|/Game/Blueprints/Tools/ToolsMaster.ToolsMaster_C|Getinfo _item)))) :!label _label)
      (else
        (bind _hasrsc (Default|RemoveRsc (Variables|Default|GetplCont) (Utilities|Struct|BreakentityStats (Variables|Default|GetentStats))))
        (if _hasrsc
          (goto _label))))))

(event EventBeginPlay
  (|CallParentFunction)
  (bind _asfp_splayer_controller (Utilities|Casting|CastToFpSPlayerController (Game|GetPlayerController 0)))
  (Variables|Default|SetplCont _asfp_splayer_controller))

(event Collision|EventActorBeginOverlap
  (params (OtherActor :type Actor%20Object%20Reference))
  (|CallParentFunction OtherActor) ; This node is disabled and will not be called.\nDrag off pins to build functionality.
)

(event EventTick
  (params (DeltaSeconds :type Float%20%28single-precision%29))
  (|CallParentFunction DeltaSeconds) ; This node is disabled and will not be called.\nDrag off pins to build functionality.
)

(fn ConstructionScript
  (|CallParentFunction))

(fn IncreaseHealth
  (params (value :type Float%20%28single-precision%29))
  (bind _output_get (Variables|Default|SetconstHealth (+ (Variables|Default|GetconstHealth) (* (/ value (.Health (Utilities|Struct|BreakentityStats (Variables|Default|GetentStats)))) 1e+02))))
  (if (> _output_get 1e+02)
    (Variables|Default|SetconstHealth 1e+02)))