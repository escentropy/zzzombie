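; Master Blueprint for a clickable building button in the farming area that opens the crafting UI for a building slot.
; On click or touch it toggles the walls crafting overlay and passes it a widget picked by ButtonId (farming, carpentry, mining, blacksmith) and the inventory's BuildId, always updating slot 0.
; SpawnBuilding replaces any existing building with a new, Z-flattened one at an offset from BuildingPos.
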(event OnClicked(planeButton)
  (params (TouchedComponent :type Primitive%20Component%20Object%20Reference) (ButtonPressed :type Key%20Structure :default "None"))
  (bind _gamemode (Variables|Default|GetgameMode))
  (bind _maingameui (Variables|/Game/Blueprints/FpSGameModeBase.FpSGameModeBase_C|GetMainGameUi _gamemode))
  (bind _wallscraftingui (Variables|/Game/UI/mainGameUi.mainGameUi_C|GetwallsCraftingUi _maingameui))
  (bind _newparam (CallFunction|GetBuilding))
  (Default|ToggeOverlay _wallscraftingui)
  (Default|UpdateBuildingsSlot _wallscraftingui 0 _newparam))

(event OnInputTouchBegin(planeButton)
  (params (FingerIndex :type ETouchIndex%20Enum :default "Touch1") (TouchedComponent :type Primitive%20Component%20Object%20Reference))
  (bind _gamemode (Variables|Default|GetgameMode))
  (bind _maingameui (Variables|/Game/Blueprints/FpSGameModeBase.FpSGameModeBase_C|GetMainGameUi _gamemode))
  (bind _wallscraftingui (Variables|/Game/UI/mainGameUi.mainGameUi_C|GetwallsCraftingUi _maingameui))
  (bind _newparam (CallFunction|GetBuilding))
  (Default|ToggeOverlay _wallscraftingui)
  (Default|UpdateBuildingsSlot _wallscraftingui 0 _newparam))

(event EventBeginPlay
  (bind _asfp_splayer_controller (Utilities|Casting|CastToFpSPlayerController (Game|GetPlayerController 0)))
  (Variables|Default|SetinvSys (Variables|/Game/Blueprints/FpSPlayerController.FpSPlayerController_C|GetinvSystem _asfp_splayer_controller))
  (bind _returnvalue (Actor|GetActorOfClass "/Game/Blueprints/Tools/craftingWidgetsBp.craftingWidgetsBp_C"))
  (Variables|Default|SetcraftingWidgetsBp _returnvalue)
  (bind _asfp_sgame_mode_base (Utilities|Casting|CastToFpSGameModeBase (Game|GetGameMode)))
  (Variables|Default|SetgameMode _asfp_sgame_mode_base))

(event Collision|EventActorBeginOverlap
  (params (OtherActor :type Actor%20Object%20Reference)))

(event EventTick
  (params (DeltaSeconds :type Float%20%28single-precision%29)))

(fn ConstructionScript)

(fn GetBuilding
  (bind _buttonid (Variables|Default|GetbuttonId))
  (bind _invsys (Variables|Default|GetinvSys))
  (bind _craftingwidgetsbp (Variables|Default|GetcraftingWidgetsBp))
  (bind _buildid (Variables|/Game/Blueprints/InventorySystem/InventorySystemBp.InventorySystemBp_C|GetbuildId _invsys))
  (bind _output (Utilities|Array|Get(acopy) _buildid _buttonid))
  (switch int _buttonid
    (:0
      (return (Utilities|Array|Get(acopy) (Variables|/Game/Blueprints/Tools/craftingWidgetsBp.craftingWidgetsBp_C|GetfarmingWidgets _craftingwidgetsbp) _output)))
    (:1
      (return (Utilities|Array|Get(acopy) (Variables|/Game/Blueprints/Tools/craftingWidgetsBp.craftingWidgetsBp_C|GetcarpentryWidgets _craftingwidgetsbp) _output)))
    (:2
      (return (Utilities|Array|Get(acopy) (Variables|/Game/Blueprints/Tools/craftingWidgetsBp.craftingWidgetsBp_C|GetminingWidgets _craftingwidgetsbp) _output)))
    (:3
      (return (Utilities|Array|Get(acopy) (Variables|/Game/Blueprints/Tools/craftingWidgetsBp.craftingWidgetsBp_C|GetblacksmithWidgets _craftingwidgetsbp) _output)))))

(fn SpawnBuilding
  (params (building :type Building%20Master%20Bp%20Object%20Reference))
  (bind _buildingpos (Variables|Default|GetbuildingPos))
  (bind _returnvalue (Transformation|GetWorldLocation _buildingpos))
  (if (Variables|Default|Getoccupied?)
    (Actor|DestroyActor (Variables|Default|GetequipedBuilding)))
  (bind _returnvalue_2 (Game|SpawnActorfromClass (Utilities|GetClass building) (Math|Transform|MakeTransform (Math|Vector|MakeVector (.x _returnvalue) (- (.y _returnvalue) 1e+02) (.z _returnvalue)) "0, 0, 0" "1.000000,1.000000,0.100000") "Undefined" 0 0))
  (Variables|Default|Setoccupied? true)
  (Variables|Default|SetequipedBuilding _returnvalue_2))