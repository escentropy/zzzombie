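; Base Blueprint for harvestable resource entities, with percentage-based health and a life-progress widget bound to the actor.
; Helper functions apply scaled damage or capped healing, count taps per tool, check and drain player stamina, and credit resources and score to FpSPlayerController.
; Tick polls health and, outside editor mode, plays particles and sound before destroying the actor at zero.
; A touchFlash event briefly shows a touch effect.
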(event Custom|touchFlash
  (bind _toucheffect (Variables|Default|GettouchEffect))
  (Rendering|SetVisibility _toucheffect true false)
  (Utilities|FlowControl|Delay 0.1)
  (Rendering|SetVisibility _toucheffect false false))

(event EventBeginPlay
  (bind _asactor_life_progress (Utilities|Casting|CastToactorLifeProgress (UserInterface|GetUserWidgetObject (Variables|Default|GetWidget))))
  (Variables|/Game/UI/actorLifeProgress.actorLifeProgress_C|SetactorOwner _asactor_life_progress self)
  (bind _asfp_splayer_controller (Utilities|Casting|CastToFpSPlayerController (Game|GetPlayerController 0)))
  (Variables|Default|SetplCont _asfp_splayer_controller)
  (Variables|Default|SetInvSysBp (Variables|/Game/Blueprints/FpSPlayerController.FpSPlayerController_C|GetinvSystem _asfp_splayer_controller)))

(event Collision|EventActorBeginOverlap
  (params (OtherActor :type Actor%20Object%20Reference)))

(event EventTick
  (params (DeltaSeconds :type Float%20%28single-precision%29))
  (bind _isdead (CallFunction|ChkDead))
  (if _isdead
    (if (not (Variables|Default|Geteditor))
      (Utilities|FlowControl|DoOnce false
        (:Completed
          (Effects|SpawnEmitteratLocation "/Game/Particles/P_MaterialFinished.P_MaterialFinished" (Transformation|GetWorldLocation (Variables|Default|GetBox)))
          (Rendering|SetVisibility (Variables|Default|GetStaticMesh) false false)
          (Audio|PlaySound2D "/Game/Sounds/ExtraSounds/Particle_sound_1_Cue.Particle_sound_1_Cue" 1.0 1.0 0.0 0 0)
          (Actor|DestroyActor))))))

(fn ConstructionScript)

(fn EntityDmg
  (params (amount :type Float%20%28single-precision%29) (health :type Float%20%28single-precision%29))
  (bind _output_get (Variables|Default|SetconstHealth (- (Variables|Default|GetconstHealth) (* (/ amount health) 1e+02))))
  (return _output_get))

(fn ChkDead
  (if (> (Variables|Default|GetconstHealth) 0.0)
    (bind _output_get (LocalVariables|Setdead false))
    (Variables|Default|SetisDead _output_get)
    (else
      (bind _output_get_2 (LocalVariables|Setdead true))
      (Variables|Default|SetisDead _output_get_2)))
  (return (LocalVariables|Getdead)))

(fn UpdateRes
  (params (resType :type resNamesEnum%20Enum :default "NewEnumerator0") (value :type Integer))
  (bind _plcont (Variables|Default|GetplCont))
  (bind _plcont_2 (Variables|Default|GetplCont))
  (bind _plcont_3 (Variables|Default|GetplCont))
  (bind _plcont_4 (Variables|Default|GetplCont))
  (bind _score (Variables|/Game/Blueprints/FpSPlayerController.FpSPlayerController_C|Getscore _plcont))
  (bind _score_2 (Variables|/Game/Blueprints/FpSPlayerController.FpSPlayerController_C|Getscore _plcont_2))
  (bind _score_3 (Variables|/Game/Blueprints/FpSPlayerController.FpSPlayerController_C|Getscore _plcont_3))
  (bind _score_4 (Variables|/Game/Blueprints/FpSPlayerController.FpSPlayerController_C|Getscore _plcont_4))
  (bind _asfp_splayer_controller (Utilities|Casting|CastToFpSPlayerController (Game|GetPlayerController 0)))
  (switch Utilities|FlowControl|Switch|SwitchonresNamesEnum resType
    (:NewEnumerator0
      (Variables|/Game/Blueprints/FpSPlayerController.FpSPlayerController_C|Setwood _asfp_splayer_controller (+ (Variables|/Game/Blueprints/FpSPlayerController.FpSPlayerController_C|Getwood _asfp_splayer_controller) value))
      (Utilities|Struct|SetmembersinscoreInfo _score_3 (+ (Utilities|Struct|BreakscoreInfo _score_3) 1)))
    (:NewEnumerator1
      (Variables|/Game/Blueprints/FpSPlayerController.FpSPlayerController_C|Setstone _asfp_splayer_controller (+ (Variables|/Game/Blueprints/FpSPlayerController.FpSPlayerController_C|Getstone _asfp_splayer_controller) value))
      (Utilities|Struct|SetmembersinscoreInfo _score_4 (+ (Utilities|Struct|BreakscoreInfo _score_4) 1)))
    (:NewEnumerator2
      (Variables|/Game/Blueprints/FpSPlayerController.FpSPlayerController_C|Setiron _asfp_splayer_controller (+ (Variables|/Game/Blueprints/FpSPlayerController.FpSPlayerController_C|Getiron _asfp_splayer_controller) value))
      (Utilities|Struct|SetmembersinscoreInfo _score (+ (Utilities|Struct|BreakscoreInfo _score) 1)))
    (:NewEnumerator4
      (Variables|/Game/Blueprints/FpSPlayerController.FpSPlayerController_C|Setfood _asfp_splayer_controller (+ (Variables|/Game/Blueprints/FpSPlayerController.FpSPlayerController_C|Getfood _asfp_splayer_controller) 1))
      (Utilities|Struct|SetmembersinscoreInfo _score_2 (+ (Utilities|Struct|BreakscoreInfo _score_2) 1)))))

(fn DecStamina
  (params (amount :type Float%20%28single-precision%29))
  (bind _asfp_splayer_controller (Utilities|Casting|CastToFpSPlayerController (Game|GetPlayerController 0)))
  (Variables|/Game/Blueprints/FpSPlayerController.FpSPlayerController_C|Setstamina _asfp_splayer_controller (- (Variables|/Game/Blueprints/FpSPlayerController.FpSPlayerController_C|Getstamina _asfp_splayer_controller) amount)))

(fn ChkStamina
  (bind _asfp_splayer_controller (Utilities|Casting|CastToFpSPlayerController (Game|GetPlayerController 0)))
  (if (> (Variables|/Game/Blueprints/FpSPlayerController.FpSPlayerController_C|Getstamina _asfp_splayer_controller) 0.0)
    (LocalVariables|Setstamina? true)
    (else
      (LocalVariables|Setstamina? false)))
  (return (LocalVariables|Getstamina?)))

(fn IncHealth
  (params (amount :type Float%20%28single-precision%29))
  (bind _output_get (Variables|Default|SetconstHealth (+ (Variables|Default|GetconstHealth) amount)))
  (if (> _output_get 1e+02)
    (Variables|Default|SetconstHealth 1e+02)
    (else
      (Variables|Default|SetconstHealth _output_get))))

(fn TapUpdate
  (params (Tool :type Tools%20Master%20Object%20Reference))
  (if (< (Variables|Default|GetcurrTap) (- (Utilities|Struct|BreaktoolsStr (Variables|/Game/Blueprints/Tools/ToolsMaster.ToolsMaster_C|Getinfo Tool)) 1))
    (Variables|Default|SetcurrTap (+ (Variables|Default|GetcurrTap) 1))
    (LocalVariables|Setready false)
    (else
      (Variables|Default|SetcurrTap 0)
      (LocalVariables|Setready true)))
  (return (LocalVariables|Getready)))

(fn IncHealthResUi
  (params (amount :type Float%20%28single-precision%29) (health :type Float%20%28single-precision%29) (level :type Integer))
  (bind _returnvalue (* level 1e+02))
  (bind _output_get (Variables|Default|SetconstHealth (+ (Variables|Default|GetconstHealth) amount)))
  (if (>= _output_get _returnvalue)
    (Variables|Default|SetconstHealth _returnvalue)
    (else
      (Variables|Default|SetconstHealth _output_get))))