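; Iron resource actor that the player harvests with the ActionInput action or by touching it.
; Either input fetches an equipped item from the inventory system and checks its type and that its id is above 1.
; A qualifying item applies its damage to the actor's health and passes its value to UpdateRes for one resource type.
; BeginPlay, overlap and Tick are disabled stubs.
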(event EventBeginPlay
  (|CallParentFunction) ; This node is disabled and will not be called.\nDrag off pins to build functionality.
)

(event Collision|EventActorBeginOverlap
  (params (OtherActor :type Actor%20Object%20Reference))
  (|CallParentFunction OtherActor) ; This node is disabled and will not be called.\nDrag off pins to build functionality.
)

(event EventTick
  (params (DeltaSeconds :type Float%20%28single-precision%29))
  (|CallParentFunction DeltaSeconds) ; This node is disabled and will not be called.\nDrag off pins to build functionality.
)

(event EventOnInputTouchBeginEvent0
  (params (FingerIndex :type ETouchIndex%20Enum :default "Touch1") (TouchedActor :type Actor%20Object%20Reference))
  (bind _item (Default|GetEquipedItem (Variables|Default|GetInvSysBp) "NewEnumerator5"))
  (if (Utilities|Enum|Equal(Enum) (.type (Variables|/Game/Blueprints/Tools/ToolsMaster.ToolsMaster_C|Getinfo _item)) "NewEnumerator1")
    (if (> (.id (Variables|/Game/Blueprints/Tools/ToolsMaster.ToolsMaster_C|Getinfo _item)) 1)
      (CallFunction|EntityDmg (Math|Conversions|ToFloat(Integer) (.dmg (Variables|/Game/Blueprints/Tools/ToolsMaster.ToolsMaster_C|Getinfo _item))) (.Health (Utilities|Struct|BreakentityStats (Variables|Default|GetentStats))))
      (CallFunction|UpdateRes "NewEnumerator2" (.value (Variables|/Game/Blueprints/Tools/ToolsMaster.ToolsMaster_C|Getinfo _item))))))

(event Input|ActionEvents|InputActionActionInput
  (params (Key :type Key%20Structure :default "None"))
  (:Pressed
    (bind _item (Default|GetEquipedItem (Variables|Default|GetInvSysBp) "NewEnumerator5"))
    (if (Utilities|Enum|Equal(Enum) (.type (Variables|/Game/Blueprints/Tools/ToolsMaster.ToolsMaster_C|Getinfo _item)) "NewEnumerator1")
      (if (> (.id (Variables|/Game/Blueprints/Tools/ToolsMaster.ToolsMaster_C|Getinfo _item)) 1)
        (CallFunction|EntityDmg (Math|Conversions|ToFloat(Integer) (.dmg (Variables|/Game/Blueprints/Tools/ToolsMaster.ToolsMaster_C|Getinfo _item))) (.Health (Utilities|Struct|BreakentityStats (Variables|Default|GetentStats))))
        (CallFunction|UpdateRes "NewEnumerator2" (.value (Variables|/Game/Blueprints/Tools/ToolsMaster.ToolsMaster_C|Getinfo _item)))))))

(fn ConstructionScript
  (|CallParentFunction))