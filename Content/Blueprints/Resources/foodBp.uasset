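; Food resource Blueprint that responds to being clicked or touched.
; Both inputs on its static mesh share one path, calling EntityDmg with damage of 100 divided by Quantity, then UpdateRes for one resource type with a value of zero.
; Tick only calls the parent, and a leftover delayed health-increment chain capped at 100 is unconnected and never runs.
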(event OnClicked(StaticMesh1)
  (params (TouchedComponent :type Primitive%20Component%20Object%20Reference) (ButtonPressed :type Key%20Structure :default "None"))
  (CallFunction|EntityDmg (Math|Conversions|ToFloat(Integer) (/ 100 (Variables|Default|Getquantity))) 1e+02)
  (CallFunction|UpdateRes "NewEnumerator4"))

(event OnInputTouchBegin(StaticMesh1)
  (params (FingerIndex :type ETouchIndex%20Enum :default "Touch1") (TouchedComponent :type Primitive%20Component%20Object%20Reference))
  (CallFunction|EntityDmg (Math|Conversions|ToFloat(Integer) (/ 100 (Variables|Default|Getquantity))) 1e+02)
  (CallFunction|UpdateRes "NewEnumerator4"))

(event EventBeginPlay
  (|CallParentFunction) ; This node is disabled and will not be called.\nDrag off pins to build functionality.
)

(event Collision|EventActorBeginOverlap
  (params (OtherActor :type Actor%20Object%20Reference))
  (|CallParentFunction OtherActor) ; This node is disabled and will not be called.\nDrag off pins to build functionality.
)

(event EventTick
  (params (DeltaSeconds :type Float%20%28single-precision%29))
  (|CallParentFunction DeltaSeconds))

(fn ConstructionScript
  (|CallParentFunction))