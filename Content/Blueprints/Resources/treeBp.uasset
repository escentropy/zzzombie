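; Harvestable tree resource actor that responds to mouse clicks and touches on its static mesh.
; Both inputs share one path that fetches the equipped item from the inventory system and checks its type.
; On a match, the item's damage is applied to the tree's health and its value is passed to a resource update.
; BeginPlay and construction only call the parent class.
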(event OnClicked(StaticMesh1)
  (params (TouchedComponent :type Primitive%20Component%20Object%20Reference) (ButtonPressed :type Key%20Structure :default "None"))
  (bind _item (Default|GetEquipedItem (Variables|Default|GetInvSysBp) "NewEnumerator5"))
  (if (Utilities|Enum|Equal(Enum) (.type (Variables|/Game/Blueprints/Tools/ToolsMaster.ToolsMaster_C|Getinfo _item)) "NewEnumerator0")
    (CallFunction|EntityDmg (Math|Conversions|ToFloat(Integer) (.dmg (Variables|/Game/Blueprints/Tools/ToolsMaster.ToolsMaster_C|Getinfo _item))) (.Health (Utilities|Struct|BreakentityStats (Variables|Default|GetentStats))))
    (CallFunction|UpdateRes "NewEnumerator0" (.value (Variables|/Game/Blueprints/Tools/ToolsMaster.ToolsMaster_C|Getinfo _item)))))

(event OnInputTouchBegin(StaticMesh1)
  (params (FingerIndex :type ETouchIndex%20Enum :default "Touch1") (TouchedComponent :type Primitive%20Component%20Object%20Reference))
  (bind _item (Default|GetEquipedItem (Variables|Default|GetInvSysBp) "NewEnumerator5"))
  (if (Utilities|Enum|Equal(Enum) (.type (Variables|/Game/Blueprints/Tools/ToolsMaster.ToolsMaster_C|Getinfo _item)) "NewEnumerator0")
    (CallFunction|EntityDmg (Math|Conversions|ToFloat(Integer) (.dmg (Variables|/Game/Blueprints/Tools/ToolsMaster.ToolsMaster_C|Getinfo _item))) (.Health (Utilities|Struct|BreakentityStats (Variables|Default|GetentStats))))
    (CallFunction|UpdateRes "NewEnumerator0" (.value (Variables|/Game/Blueprints/Tools/ToolsMaster.ToolsMaster_C|Getinfo _item)))))

(event EventBeginPlay
  (|CallParentFunction))

(event Collision|EventActorBeginOverlap
  (params (OtherActor :type Actor%20Object%20Reference))
  (|CallParentFunction OtherActor) ; This node is disabled and will not be called.\nDrag off pins to build functionality.
)

(event EventTick
  (params (DeltaSeconds :type Float%20%28single-precision%29))
  (|CallParentFunction DeltaSeconds) ; This node is disabled and will not be called.\nDrag off pins to build functionality.
)

(fn ConstructionScript
  (|CallParentFunction))