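; Tree resource actor that the player harvests by clicking its static mesh.
; On click, it reads the item at index 0 from the inventory system and passes that item's damage stat to EntityDmg.
; The same click calls UpdateRes with the first resource type and the item's value.
; All other lifecycle events are disabled stubs, and the construction script only calls its parent.
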(event OnClicked(StaticMesh)
  (params (TouchedComponent :type Primitive%20Component%20Object%20Reference) (ButtonPressed :type Key%20Structure :default "None"))
  (bind _item (Default|GetItem (Variables|Default|GetInvSysBp)))
  (CallFunction|EntityDmg (Math|Conversions|ToFloat(Integer) (.dmg (Variables|/Game/Blueprints/Tools/ToolsMaster.ToolsMaster_C|Getinfo _item))))
  (CallFunction|UpdateRes "NewEnumerator0" (.value (Variables|/Game/Blueprints/Tools/ToolsMaster.ToolsMaster_C|Getinfo _item))))

(event EventBeginPlay
  (|CallParentFunction) ; This node is disabled and will not be called.\nDrag off pins to build functionality.
)

(event Collision|EventActorBeginOverlap
  (params (OtherActor :type Actor%20Object%20Reference))
  (|CallParentFunction OtherActor) ; This node is disabled and will not be called.\nDrag off pins to build functionality.
)

(event EventTick
  (params (DeltaSeconds :type Float%20%28single-precision%29))
  (|CallParentFunction DeltaSeconds) ; This node is disabled and will not be called.\nDrag off pins to build functionality.
)

(fn ConstructionScript
  (|CallParentFunction))