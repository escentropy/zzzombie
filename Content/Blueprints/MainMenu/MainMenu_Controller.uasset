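; Main menu controller that gates creation of the menu widgets behind a platform login, noted as Google login.
; On BeginPlay it checks whether the first player is logged in and otherwise shows the external login UI.
; An existing or successful login creates and stores the main menu, leaderboard and settings widgets, without adding them to the viewport here.
; A failed login only prints a string, leaving the widgets uncreated.
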(event EventBeginPlay
  (bind _returnvalue (Game|GetPlayerController 0))
  ;[1 1 1] Google Login
  (if (Class|KismetSystemLibrary|IsLoggedin _returnvalue)
    (bind _returnvalue_2 (UserInterface|CreateWidget "/Game/UI/MainMenuUI.MainMenuUI_C" :!label _label))
    (Variables|Default|SetMainMenuUI _returnvalue_2)
    (bind _returnvalue_3 (UserInterface|CreateWidget "/Game/UI/Leaderboard/Leaderboard_ui.Leaderboard_ui_C"))
    (Variables|Default|SetLeaderBoardUI _returnvalue_3)
    (bind _returnvalue_4 (UserInterface|CreateWidget "/Game/UI/Settings.Settings_C" 0 3))
    (Variables|Default|Setsettings _returnvalue_4)
    (else
      (|ShowExternalLoginUI _returnvalue
        (:OnSuccess
          (Development|PrintString "Hello")
          (goto _label))
        (:OnFailure
          (Development|PrintString "Hello"))))))

(fn ConstructionScript)