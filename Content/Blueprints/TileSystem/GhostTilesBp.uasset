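; GhostTilesBp is a tile-system Blueprint that lays out a flat grid of static mesh tiles.
; Its construction script loops over GridX and GridY, adding a mesh component per cell at multiples of Spacing and storing each in TileMeshes.
; GridX counts tiles along local Y and GridY along local X.
; The event graph holds only disabled default events, so it has no runtime logic.
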(event EventBeginPlay)

(event Collision|EventActorBeginOverlap
  (params (OtherActor :type Actor%20Object%20Reference)))

(event EventTick
  (params (DeltaSeconds :type Float%20%28single-precision%29)))

(fn ConstructionScript
  (bind _spacing (Variables|Default|Getspacing))
  (for _index (range 0 (- (Variables|Default|GetgridX) 1))
    (for _index_2 (range 0 (- (Variables|Default|GetgridY) 1))
      (bind _returnvalue (AddComponent|AddStaticMeshComponent false (Math|Transform|MakeTransform (Math|Vector|MakeVector (* _index_2 _spacing) (* _index _spacing) 0.0))))
      (Utilities|Array|Add (Variables|Default|GettileMeshes) _returnvalue))))