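; Board tile actor that holds placed traps and can regenerate resources during the daytime.
; Tick drives a once-per-day check that, at a randomized day interval, rarely spawns one of two resources from CraftingWidgetsBp on free, zombie-clear tiles.
; spawnTrap applies the same clearance checks, charges the player controller, then uses SpawnEntity to mark the tile occupied and pass it the board Id.
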(event Custom|Regeneration
  (bind _gamemode (Variables|Default|GetgameMode))
  (if (Variables|/Game/Blueprints/FpSGameModeBase.FpSGameModeBase_C|GetDay? _gamemode)
    (Utilities|FlowControl|DoOnce false :!label _label
      (:Completed
        (if (== (* (Variables|Default|GetgenDays) (Variables|Default|GetgenIncr)) (Variables|/Game/Blueprints/FpSGameModeBase.FpSGameModeBase_C|GetnumDays _gamemode))
          (Variables|Default|SetgenIncr (+ (Variables|Default|GetgenIncr) 1))
          (if (not (Variables|Default|Getoccupied))
            (if (== (Utilities|Array|Length (Collision|GetOverlappingActors (Variables|Default|GetcheckSouround) "/Game/Blueprints/enemy/enemyZombie.enemyZombie_C" :!class /Script/Engine.PrimitiveComponent)) 0)
              (if (> (Math|Random|RandomIntegerinRange 0 100) 97)
                (Utilities|FlowControl|DoOnce false :!label _label_2
                  (:Completed
                    (Game|SpawnActorfromClass (Utilities|GetClass (Utilities|Array|Get(acopy) (Variables|Default|Getresources) (Math|Random|RandomIntegerinRange 0 1))) (Math|Transform|MakeTransform (Transformation|GetWorldLocation (Variables|Default|GetspawnVector)) "0, 0, 0" "1,1,1") "Undefined" 0 0)))
                (else
                  (goto _label_2 Reset))))))))
    (else
      (goto _label Reset))))

(event Custom|spawnTrap
  (params (trap :type Trap%20Master%20Object%20Reference))
  (if (not (Variables|Default|Getoccupied))
    (if (== (Utilities|Array|Length (Collision|GetOverlappingActors (Variables|Default|GetcheckSouround) "/Game/Blueprints/enemy/enemyZombie.enemyZombie_C" :!class /Script/Engine.PrimitiveComponent)) 0)
      (bind _hasrsc (Default|RemoveRsc (Variables|Default|GetplCont) (.Cost (Utilities|Struct|BreakentityStats (Variables|/Game/Blueprints/Resources/entityMasterBp.entityMasterBp_C|GetentStats trap)))))
      (if _hasrsc
        (CallFunction|SpawnEntity (Math|Transform|MakeTransform (Transformation|GetWorldLocation (Variables|Default|GetspawnVector)) "0, 0, 0" "1,1,1") (Utilities|GetClass trap))))))

(event EventBeginPlay
  (bind _astile_slot_ui (Utilities|Casting|CastTotileSlotUi (UserInterface|GetUserWidgetObject (Variables|Default|GetWidget))))
  (Variables|/Game/UI/TrapUi/tileSlotUi.tileSlotUi_C|Settile _astile_slot_ui self)
  (Utilities|FlowControl|Delay 0.2)
  (bind _asfp_sgame_mode_base (Utilities|Casting|CastToFpSGameModeBase (Game|GetGameMode)))
  (Variables|Default|SetgameMode _asfp_sgame_mode_base)
  (Variables|Default|SetgenDays (Math|Random|RandomIntegerinRange (Variables|Default|GetgenDays) (* (Variables|Default|GetgenDays) 2)))
  (bind _returnvalue (Actor|GetActorOfClass "/Game/Blueprints/Tools/craftingWidgetsBp.craftingWidgetsBp_C"))
  (Variables|Default|Setresources (Variables|/Game/Blueprints/Tools/craftingWidgetsBp.craftingWidgetsBp_C|GetresourcesBp _returnvalue))
  (bind _asfp_splayer_controller (Utilities|Casting|CastToFpSPlayerController (Game|GetPlayerController 0)))
  (Variables|Default|SetplCont _asfp_splayer_controller))

(event Collision|EventActorBeginOverlap
  (params (OtherActor :type Actor%20Object%20Reference)))

(event EventTick
  (params (DeltaSeconds :type Float%20%28single-precision%29))
  (Utilities|FlowControl|Sequence
    (:then_0
      (Utilities|FlowControl|Delay 0.2)
      (CallFunction|Regeneration))))

(fn ConstructionScript)

(fn SpawnEntity
  (params (InLocation :type Transform) (Class :type Actor%20Class%20Reference))
  (bind _returnvalue (Game|SpawnActorfromClass Class InLocation "Undefined" 0 0))
  (Variables|Default|Setoccupied true)
  (bind _asentity_master_bp (Utilities|Casting|CastToentityMasterBp _returnvalue))
  (bind _output_get (Variables|Default|SetentityOccupied _asentity_master_bp))
  (Variables|/Game/Blueprints/Resources/entityMasterBp.entityMasterBp_C|SetboardId _asentity_master_bp (Variables|Default|Getid))
  (return _output_get))