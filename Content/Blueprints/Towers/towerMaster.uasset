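; Base defensive tower that damages zombies in a level-specific fire area and can be repaired by the player.
; Its ID selects the fire area actor at BeginPlay.
; A Delay on Tick paces attacks on an enemy chosen by comparing X positions, falling back to the first overlap.
; Click or touch with the right equipped item type restores percentage health, costing resources outside debug mode.
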(event OnClicked(StaticMesh1)
  (params (TouchedComponent :type Primitive%20Component%20Object%20Reference) (ButtonPressed :type Key%20Structure :default "None"))
  ;[1 1 1] OnClicked
  (bind _returnvalue (Actor|GetActorOfClass "/Game/Blueprints/DebugModeBp.DebugModeBp_C"))
  (bind _item (Default|GetEquipedItem (Variables|Default|GetInvSysBp) "NewEnumerator5"))
  (if (Utilities|Enum|Equal(Enum) (.Type (Utilities|Struct|BreaktoolsStr (Variables|/Game/Blueprints/Tools/ToolsMaster.ToolsMaster_C|Getinfo _item))) "NewEnumerator4")
    (if (Variables|/Game/Blueprints/DebugModeBp.DebugModeBp_C|Getdebug? _returnvalue)
      (CallFunction|IncreaseHelath (Math|Conversions|ToFloat(Integer) (.value (Utilities|Struct|BreaktoolsStr (Variables|/Game/Blueprints/Tools/ToolsMaster.ToolsMaster_C|Getinfo _item)))) 0.0 :!label _label)
      (Audio|PlaySound2D (.Sound (Utilities|Struct|BreaktoolsStr (Variables|/Game/Blueprints/Tools/ToolsMaster.ToolsMaster_C|Getinfo _item))) 1.0 1.0 0.0 0 0)
      (else
        (bind _hasrsc (Default|RemoveRsc (Variables|Default|GetplCont) (Utilities|Struct|BreakentityStats (Variables|Default|GetentStats))))
        (if _hasrsc
          (goto _label))))))

(event OnInputTouchBegin(StaticMesh1)
  (params (FingerIndex :type ETouchIndex%20Enum :default "Touch1") (TouchedComponent :type Primitive%20Component%20Object%20Reference))
  ;[1 1 1] OnClicked
  (bind _returnvalue (Actor|GetActorOfClass "/Game/Blueprints/DebugModeBp.DebugModeBp_C"))
  (bind _item (Default|GetEquipedItem (Variables|Default|GetInvSysBp) "NewEnumerator5"))
  (if (Utilities|Enum|Equal(Enum) (.Type (Utilities|Struct|BreaktoolsStr (Variables|/Game/Blueprints/Tools/ToolsMaster.ToolsMaster_C|Getinfo _item))) "NewEnumerator4")
    (if (Variables|/Game/Blueprints/DebugModeBp.DebugModeBp_C|Getdebug? _returnvalue)
      (CallFunction|IncreaseHelath (Math|Conversions|ToFloat(Integer) (.value (Utilities|Struct|BreaktoolsStr (Variables|/Game/Blueprints/Tools/ToolsMaster.ToolsMaster_C|Getinfo _item)))) 0.0 :!label _label)
      (Audio|PlaySound2D (.Sound (Utilities|Struct|BreaktoolsStr (Variables|/Game/Blueprints/Tools/ToolsMaster.ToolsMaster_C|Getinfo _item))) 1.0 1.0 0.0 0 0)
      (else
        (bind _hasrsc (Default|RemoveRsc (Variables|Default|GetplCont) (Utilities|Struct|BreakentityStats (Variables|Default|GetentStats))))
        (if _hasrsc
          (goto _label))))))

(event EventBeginPlay
  (|CallParentFunction)
  (CallFunction|SetFireArea)
  (bind _asfp_splayer_controller (Utilities|Casting|CastToFpSPlayerController (Game|GetPlayerController 0)))
  (Variables|Default|SetplCont _asfp_splayer_controller)
  (bind _returnvalue (Actor|GetActorOfClass "/Game/Blueprints/Tools/craftingWidgetsBp.craftingWidgetsBp_C"))
  (Variables|Default|SetcraftWidgetsBp _returnvalue))

(event Collision|EventActorBeginOverlap
  (params (OtherActor :type Actor%20Object%20Reference))
  (|CallParentFunction OtherActor) ; This node is disabled and will not be called.\nDrag off pins to build functionality.
)

(event EventTick
  (params (DeltaSeconds :type Float%20%28single-precision%29))
  (bind _firearea (Variables|Default|GetfireArea))
  (bind _firearea_2 (Variables|/Game/Blueprints/Towers/FireArea/fireAreaMaster.fireAreaMaster_C|GetfireArea _firearea))
  (bind _overlappingactors (Collision|GetOverlappingActors _firearea_2 "/Game/Blueprints/enemy/enemyZombie.enemyZombie_C" :!class /Script/Engine.PrimitiveComponent))
  ;[1 1 1] Tick
  (|CallParentFunction DeltaSeconds)
  (if (not (Variables|Default|Geteditor))
    (Utilities|FlowControl|Delay 2.0)
    (for _array_element _overlappingactors
      (bind _asenemy_zombie (Utilities|Casting|CastToenemyZombie _array_element))
      (bind _array_element_2 (Utilities|Array|ForEachLoopwithBreak _overlappingactors :!label _label)
        (:LoopBody
          (bind _asenemy_zombie_2 (Utilities|Casting|CastToenemyZombie _array_element_2))
          (if (< (.x (Transformation|GetWorldLocation (Variables|/Game/Blueprints/enemy/enemyZombie.enemyZombie_C|GetSkeletalMesh _asenemy_zombie))) (.x (Transformation|GetWorldLocation (Variables|/Game/Blueprints/enemy/enemyZombie.enemyZombie_C|GetSkeletalMesh _asenemy_zombie_2))))
            (Variables|Default|SetclosestEnemy _asenemy_zombie)
            (else
              (goto _label Break))))))
    (if (Utilities|IsValid (Variables|Default|GetclosestEnemy))
      (Default|EntityHit (Variables|Default|GetclosestEnemy) 1e+01)
      (else
        (bind _asenemy_zombie_3 (Utilities|Casting|CastToenemyZombie (Utilities|Array|Get(acopy) _overlappingactors)))
        (Default|EntityHit _asenemy_zombie_3 1e+01)))))

(fn ConstructionScript
  (|CallParentFunction))

(fn IncreaseHelath
  (params (value :type Float%20%28single-precision%29) (health :type Float%20%28single-precision%29))
  (bind _output_get (Variables|Default|SetconstHealth (+ (Variables|Default|GetconstHealth) (* (/ value (.Health (Utilities|Struct|BreakentityStats (Variables|Default|GetentStats)))) 1e+02))))
  (if (> _output_get 1e+02)
    (Variables|Default|SetconstHealth 1e+02)))

(fn ChangeMaterial
  (Components|StaticMesh|SetStaticMesh (Variables|Default|GetStaticMesh) (Utilities|Array|Get(acopy) (Variables|/Game/Blueprints/Tools/craftingWidgetsBp.craftingWidgetsBp_C|GetwallMeshes (Variables|Default|GetcraftWidgetsBp)) (.id (Utilities|Struct|BreaktoolsStr (Variables|Default|Getinfo))))))

(fn SetFireArea
  (switch int (Utilities|Struct|BreaktoolsStr (Variables|Default|Getinfo))
    (:0
      (bind _returnvalue (Actor|GetActorOfClass "/Game/Blueprints/Towers/FireArea/fireAreaLevel1.fireAreaLevel1_C"))
      (Variables|Default|SetfireArea _returnvalue))
    (:1
      (bind _returnvalue_2 (Actor|GetActorOfClass "/Game/Blueprints/Towers/FireArea/fireAreaLevel2.fireAreaLevel2_C"))
      (Variables|Default|SetfireArea _returnvalue_2))
    (:2
      (bind _returnvalue_3 (Actor|GetActorOfClass "/Game/Blueprints/Towers/FireArea/fireAreaLevel3.fireAreaLevel3_C"))
      (Variables|Default|SetfireArea _returnvalue_3))))