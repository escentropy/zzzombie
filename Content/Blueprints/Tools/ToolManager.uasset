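; Tool manager that creates the tool and weapon objects for five categories: axes, pickaxes, melee, ranged and hammers.
; Each category has its own function that constructs objects owned by the manager and stores them in that category's array.
; Every array starts with an empty-hands entry followed by three tiers: wood, stone and iron, or slingshot, bow and crossbow for ranged.
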(fn CreateAxeObjs
  (bind _returnvalue (Game|ConstructObjectfromClass "/Game/Blueprints/Tools/emtyHands.emtyHands_C" self))
  (bind _returnvalue_2 (Game|ConstructObjectfromClass "/Game/Blueprints/Tools/Axes/woodenAxeBp.woodenAxeBp_C" self))
  (bind _returnvalue_3 (Game|ConstructObjectfromClass "/Game/Blueprints/Tools/Axes/stoneAxeBp.stoneAxeBp_C" self))
  (bind _returnvalue_4 (Game|ConstructObjectfromClass "/Game/Blueprints/Tools/Axes/ironAxeBp.ironAxeBp_C" self))
  (Variables|Default|Setaxes (Utilities|Array|MakeArray _returnvalue _returnvalue_2 _returnvalue_3 _returnvalue_4)))

(fn CreatePickaxeObjs
  (bind _returnvalue (Game|ConstructObjectfromClass "/Game/Blueprints/Tools/emtyHands.emtyHands_C" self))
  (bind _returnvalue_2 (Game|ConstructObjectfromClass "/Game/Blueprints/Tools/Pickaxes/woodenPickBp.woodenPickBp_C" self))
  (bind _returnvalue_3 (Game|ConstructObjectfromClass "/Game/Blueprints/Tools/Pickaxes/stonePickBp.stonePickBp_C" self))
  (bind _returnvalue_4 (Game|ConstructObjectfromClass "/Game/Blueprints/Tools/Pickaxes/ironPickBp.ironPickBp_C" self))
  (Variables|Default|Setpickaxes (Utilities|Array|MakeArray _returnvalue _returnvalue_2 _returnvalue_3 _returnvalue_4)))

(fn CreateMeleeObjs
  (bind _returnvalue (Game|ConstructObjectfromClass "/Game/Blueprints/Tools/emtyHands.emtyHands_C" self))
  (bind _returnvalue_2 (Game|ConstructObjectfromClass "/Game/Blueprints/Tools/Mellee/woodenSwordBp.woodenSwordBp_C" self))
  (bind _returnvalue_3 (Game|ConstructObjectfromClass "/Game/Blueprints/Tools/Mellee/stoneSwordBp.stoneSwordBp_C" self))
  (bind _returnvalue_4 (Game|ConstructObjectfromClass "/Game/Blueprints/Tools/Mellee/ironSwoordBp.ironSwoordBp_C" self))
  (Variables|Default|Setmelees (Utilities|Array|MakeArray _returnvalue _returnvalue_2 _returnvalue_3 _returnvalue_4)))

(fn CreateRangeObjs
  (bind _returnvalue (Game|ConstructObjectfromClass "/Game/Blueprints/Tools/emtyHands.emtyHands_C" self))
  (bind _returnvalue_2 (Game|ConstructObjectfromClass "/Game/Blueprints/Tools/Range/slingshotBp.slingshotBp_C" self))
  (bind _returnvalue_3 (Game|ConstructObjectfromClass "/Game/Blueprints/Tools/Range/BowBp.BowBp_C" self))
  (bind _returnvalue_4 (Game|ConstructObjectfromClass "/Game/Blueprints/Tools/Range/crossbowBp.crossbowBp_C" self))
  (Variables|Default|Setranges (Utilities|Array|MakeArray _returnvalue _returnvalue_2 _returnvalue_3 _returnvalue_4)))

(fn CreateHammerObjs
  (bind _returnvalue (Game|ConstructObjectfromClass "/Game/Blueprints/Tools/emtyHands.emtyHands_C" self))
  (bind _returnvalue_2 (Game|ConstructObjectfromClass "/Game/Blueprints/Tools/hammers/woodenHammer.woodenHammer_C" self))
  (bind _returnvalue_3 (Game|ConstructObjectfromClass "/Game/Blueprints/Tools/hammers/stoneHameer.stoneHameer_C" self))
  (bind _returnvalue_4 (Game|ConstructObjectfromClass "/Game/Blueprints/Tools/hammers/ironHammer.ironHammer_C" self))
  (Variables|Default|Sethammers (Utilities|Array|MakeArray _returnvalue _returnvalue_2 _returnvalue_3 _returnvalue_4)))