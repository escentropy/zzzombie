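; Helper Blueprint that pre-builds the crafting UI slot widgets for tools, traps and buildings at game start.
; After a short delay, BeginPlay caches the main GUI, then fills per-category widget arrays from ToolManager lists, TrapMaster actors in the level and building arrays.
; It also gathers a combined AllTools list, skipping each category's first entry except for axes, and sets resource icons.
; A wall-gathering function exists but is never called here.
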(event EventBeginPlay
  (bind _asfp_splayer_controller (Utilities|Casting|CastToFpSPlayerController (Game|GetPlayerController 0)))
  (bind _output_get (Variables|Default|SetplaCont _asfp_splayer_controller))
  (Variables|Default|SettoolManager (Variables|/Game/Blueprints/FpSPlayerController.FpSPlayerController_C|GettoolManager _output_get))
  (Utilities|FlowControl|Delay 0.2)
  (bind _asfp_sgame_mode_base (Utilities|Casting|CastToFpSGameModeBase (Game|GetGameMode)))
  (Variables|Default|SetmainGui (Variables|/Game/Blueprints/FpSGameModeBase.FpSGameModeBase_C|GetMainGameUi _asfp_sgame_mode_base))
  (CallFunction|CreateTrapCrWid)
  (CallFunction|CreateToolCraftingWidgets)
  (CallFunction|CreateBuildingsWidgets)
  (CallFunction|CreateResourceImages))

(fn ConstructionScript)

(fn CreateToolCraftingWidgets
  (bind _toolmanager (Variables|Default|GettoolManager))
  (bind _maingui (Variables|Default|GetmainGui))
  (Utilities|FlowControl|Sequence
    (:then_0
      (for (_array_element _array_index) (Variables|/Game/Blueprints/Tools/ToolManagerBp.ToolManagerBp_C|Getaxes _toolmanager)
        (bind _returnvalue (UserInterface|CreateWidget "/Game/UI/craftingSlot.craftingSlot_C" 0 _maingui _array_element))
        (Utilities|Array|Add (Variables|Default|GetaxeCraftingSlots) _returnvalue)
        (Utilities|Array|Add (Variables|Default|GetallTools) _array_element)))
    (:then_1
      (for (_array_element_2 _array_index_2) (Variables|/Game/Blueprints/Tools/ToolManagerBp.ToolManagerBp_C|Getpickaxes _toolmanager)
        (bind _returnvalue_2 (UserInterface|CreateWidget "/Game/UI/craftingSlot.craftingSlot_C" 0 _maingui _array_element_2 "NewEnumerator1"))
        (Utilities|Array|Add (Variables|Default|GetpickCraftingSlots) _returnvalue_2)
        (if (> _array_index_2 0)
          (Utilities|Array|Add (Variables|Default|GetallTools) _array_element_2))))
    (:then_2
      (for (_array_element_3 _array_index_3) (Variables|/Game/Blueprints/Tools/ToolManagerBp.ToolManagerBp_C|Getmelees _toolmanager)
        (bind _returnvalue_3 (UserInterface|CreateWidget "/Game/UI/craftingSlot.craftingSlot_C" 0 _maingui _array_element_3 "NewEnumerator2"))
        (Utilities|Array|Add (Variables|Default|GetmeleeCraftingSlots) _returnvalue_3)
        (if (> _array_index_3 0)
          (Utilities|Array|Add (Variables|Default|GetallTools) _array_element_3))))
    (:then_3
      (for (_array_element_4 _array_index_4) (Variables|/Game/Blueprints/Tools/ToolManagerBp.ToolManagerBp_C|Getranges _toolmanager)
        (bind _returnvalue_4 (UserInterface|CreateWidget "/Game/UI/craftingSlot.craftingSlot_C" 0 _maingui _array_element_4 "NewEnumerator3"))
        (Utilities|Array|Add (Variables|Default|GetrangeCraftingSlots) _returnvalue_4)
        (if (> _array_index_4 0)
          (Utilities|Array|Add (Variables|Default|GetallTools) _array_element_4))))
    (:then_4
      (for (_array_element_5 _array_index_5) (Variables|/Game/Blueprints/Tools/ToolManagerBp.ToolManagerBp_C|Gethammers _toolmanager)
        (bind _returnvalue_5 (UserInterface|CreateWidget "/Game/UI/craftingSlot.craftingSlot_C" 0 _maingui _array_element_5 "NewEnumerator4"))
        (Utilities|Array|Add (Variables|Default|GethammerCraftingSlots) _returnvalue_5)
        (if (> _array_index_5 0)
          (Utilities|Array|Add (Variables|Default|GetallTools) _array_element_5))))))

(fn CreateTrapCrWid
  (CallFunction|CreateTrapsBp)
  (for _array_element (Variables|Default|GettrapsBp)
    (bind _returnvalue (UserInterface|CreateWidget "/Game/UI/TrapUi/trapSlotUi.trapSlotUi_C" 0 _array_element))
    (Utilities|Array|Add (Variables|Default|GettrapWidgets) _returnvalue)))

(fn CreateTrapsBp
  (bind _outactors (Actor|GetAllActorsOfClass "/Game/Blueprints/Traps/TrapMaster.TrapMaster_C"))
  (Variables|Default|SettrapsBp _outactors))

(fn CreateWallsBp
  (bind _outactors (Actor|GetAllActorsOfClass "/Game/Blueprints/Walls/wallsMaster.wallsMaster_C"))
  (bind _arrayelement (Utilities|Array|ReverseforEachLoop _outactors)
    (:LoopBody
      (Utilities|Array|Add (Variables|Default|GetwallsBp) _arrayelement))))

(fn CreateBuildingsWidgets
  (Utilities|FlowControl|Sequence
    (:then_0
      (for _array_element (Variables|Default|GetfarmingBp)
        (bind _returnvalue (UserInterface|CreateWidget "/Game/UI/buildingCraftingSlotUi.buildingCraftingSlotUi_C" 0 0 (Variables|Default|GetmainGui) _array_element))
        (Utilities|Array|Add (Variables|Default|GetfarmingWidgets) _returnvalue)))
    (:then_1
      (for _array_element_2 (Variables|Default|GetcarpentryBp)
        (bind _returnvalue_2 (UserInterface|CreateWidget "/Game/UI/buildingCraftingSlotUi.buildingCraftingSlotUi_C" 0 1 (Variables|Default|GetmainGui) _array_element_2))
        (Utilities|Array|Add (Variables|Default|GetcarpentryWidgets) _returnvalue_2)))
    (:then_2
      (for _array_element_3 (Variables|Default|GetminingBp)
        (bind _returnvalue_3 (UserInterface|CreateWidget "/Game/UI/buildingCraftingSlotUi.buildingCraftingSlotUi_C" 0 2 (Variables|Default|GetmainGui) _array_element_3))
        (Utilities|Array|Add (Variables|Default|GetminingWidgets) _returnvalue_3)))
    (:then_3
      (for _array_element_4 (Variables|Default|GetblacksmithBp)
        (bind _returnvalue_4 (UserInterface|CreateWidget "/Game/UI/buildingCraftingSlotUi.buildingCraftingSlotUi_C" 0 3 (Variables|Default|GetmainGui) _array_element_4))
        (Utilities|Array|Add (Variables|Default|GetblacksmithWidgets) _returnvalue_4)))))

(fn CreateResourceImages
  (Variables|Default|SetresImgs (Utilities|Array|MakeArray "/Game/UI/UI_Images/Icons/corn_icon.corn_icon" "/Game/UI/UI_Images/Icons/wood_icon.wood_icon" "/Game/UI/UI_Images/Icons/stone_icon.stone_icon" "/Game/UI/UI_Images/Icons/iron_icon.iron_icon")))