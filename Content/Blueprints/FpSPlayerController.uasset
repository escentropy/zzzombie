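; Player controller for a survival game that holds the player's health, hunger, resources and score stats.
; Construction builds the inventory and tool manager; BeginPlay creates widgets, then loads saved stats from the GameInstance or DebugMode resources.
; Tick drains hunger on a speed-scaled delay, auto-eats food, damages health when starving and triggers game over.
; It also provides resource cost checks, damage/kill-rate tracking, a market hotkey and layered Android Back menu handling.
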(event Custom|LoadResources
  (CallFunction|LoadInfo))

(event Custom|Kills/Min
  ;[1 1 1] Kills/Minute
  (CallFunction|Kls/mnt))

(event Custom|Dmg/Minute
  (params (dmg :type Float%20%28single-precision%29))
  ;[1 1 1] dmg/minute
  (CallFunction|Dmg/min dmg))

(event EventBeginPlay
  ;[1 1 1] BeginPlay
  (CallFunction|CreateWidgets)
  (CallFunction|CreateObjs)
  (if (Variables|/Game/Blueprints/GameInstanceBp.GameInstanceBp_C|Getcontinue (Variables|Default|GetgameInstance))
    (CallFunction|LoadResources)
    (else
      (bind _returnvalue (Game|GetCurrentLevelName true))
      (if (Utilities|Enum|Equal(Enum) _returnvalue "MainGameLevel")
        (CallFunction|DefaultResources)))))

(event EventTick
  (params (DeltaSeconds :type Float%20%28single-precision%29))
  ;[1 1 1] Tick
  (Utilities|FlowControl|Sequence
    (:then_0
      (Utilities|FlowControl|Delay (/ (Variables|Default|GetconstHungerRatio) (Variables|/Game/Blueprints/FpSGameModeBase.FpSGameModeBase_C|GetglobalSpeed (Variables|Default|GetgameMode))))
      (if (> (Variables|Default|Gethunger) 0.0)
        (Variables|Default|Sethunger (- (Variables|Default|Gethunger) 0.01))
        (if (< (Variables|Default|Gethunger) 9e+01)
          (if (> (Variables|Default|Getfood) 0)
            (Utilities|FlowControl|DoOnce false :!label _label
              (:Completed
                (Variables|Default|Sethunger (Math|Conversions|ToFloat(Integer) (+ (Math|Float|Truncate (Variables|Default|Gethunger)) 10)))
                (Variables|Default|Setfood (- (Variables|Default|Getfood) 1))
                (goto _label Reset)))))
        (else
          (Variables|Default|Sethealth (- (Variables|Default|Gethealth) 0.05)))))
    (:then_1
      (if (not (> (Variables|Default|Gethealth) 0.0))
        (CallFunction|GameOver)))))

(event Input|KeyboardEvents|AndroidBack
  (params (Key :type Key%20Structure :default "None"))
  ;[1 1 1] Android Back
  (:Pressed
    (CallFunction|AndroidBack)))

(event Input|KeyboardEvents|M
  (params (Key :type Key%20Structure :default "None"))
  (:Pressed
    (UserInterface|Viewport|AddtoViewport (Variables|Default|GetmarketUi) 0)))

(event Input|KeyboardEvents|Backspace
  (params (Key :type Key%20Structure :default "None"))
  (:Pressed
    ;[1 1 1] Android Back
    (CallFunction|AndroidBack)))

(fn ConstructionScript
  (bind _returnvalue (Game|ConstructObjectfromClass "/Game/Blueprints/InventorySystem/InventorySystemBp.InventorySystemBp_C" self))
  (bind _output_get (Variables|Default|SetinvSystem _returnvalue))
  (bind _returnvalue_2 (Game|ConstructObjectfromClass "/Game/Blueprints/Tools/ToolManagerBp.ToolManagerBp_C" self))
  (bind _output_get_2 (Variables|Default|SettoolManager _returnvalue_2))
  (Variables|/Game/Blueprints/InventorySystem/InventorySystemBp.InventorySystemBp_C|SettoolManager _output_get _output_get_2)
  (CallFunction|CreateToolObjs))

(fn CreateToolObjs
  (bind _toolmanager (Variables|Default|GettoolManager))
  (Default|CreateAxeObjs _toolmanager)
  (Default|CreatePickaxeObjs _toolmanager)
  (Default|CreateMeleeObjs _toolmanager)
  (Default|CreateRangeObjs _toolmanager)
  (Default|CreateHammerObjs _toolmanager))

(fn RemoveRsc
  (params (cost :type Ent%20Cost%20Structure))
  (bind (_wood _stone _iron _food) (Utilities|Struct|BreakentCost cost))
  (Utilities|FlowControl|Sequence
    (:then_0
      (if (>= (Variables|Default|Getwood) _wood)
        (LocalVariables|Sethas? true)
        (else
          (LocalVariables|Sethas? false)
          (return (LocalVariables|Gethas?)))))
    (:then_1
      (if (>= (Variables|Default|Getstone) _stone)
        (LocalVariables|Sethas? true)
        (else
          (LocalVariables|Sethas? false)
          (return (LocalVariables|Gethas?)))))
    (:then_2
      (if (>= (Variables|Default|Getiron) _iron)
        (LocalVariables|Sethas? true)
        (else
          (LocalVariables|Sethas? false)
          (return (LocalVariables|Gethas?)))))
    (:then_3
      (if (>= (Variables|Default|Getfood) _food)
        (LocalVariables|Sethas? true)
        (else
          (LocalVariables|Sethas? false)
          (return (LocalVariables|Gethas?)))))
    (:then_4
      (Variables|Default|Setwood (- (Variables|Default|Getwood) _wood))
      (Variables|Default|Setstone (- (Variables|Default|Getstone) _stone))
      (Variables|Default|Setiron (- (Variables|Default|Getiron) _iron))
      (Variables|Default|Setfood (- (Variables|Default|Getfood) _food))
      (return (LocalVariables|Gethas?)))))

(fn DefaultResources
  (bind _returnvalue (Actor|GetActorOfClass "/Game/Blueprints/DebugModeBp.DebugModeBp_C"))
  (bind _output_get (Variables|Default|SetdebugMode _returnvalue))
  (if (Variables|/Game/Blueprints/DebugModeBp.DebugModeBp_C|Getdebug? _output_get)
    (Variables|Default|Setfood (Variables|/Game/Blueprints/DebugModeBp.DebugModeBp_C|GetFood _output_get))
    (Variables|Default|Setwood (Variables|/Game/Blueprints/DebugModeBp.DebugModeBp_C|GetWood _output_get))
    (Variables|Default|Setstone (Variables|/Game/Blueprints/DebugModeBp.DebugModeBp_C|GetStone _output_get))
    (Variables|Default|Setiron (Variables|/Game/Blueprints/DebugModeBp.DebugModeBp_C|GetIron _output_get))
    (Variables|Default|Setcoins (Variables|/Game/Blueprints/DebugModeBp.DebugModeBp_C|Getcoins _output_get))))

(fn CreateObjs
  (bind _returnvalue (UserInterface|CreateWidget "/Game/UI/Market/marketUi.marketUi_C" 0 self))
  (Variables|Default|SetmarketUi _returnvalue)
  (bind _asgame_instance_bp (Utilities|Casting|CastToGameInstanceBp (Game|GetGameInstance)))
  (Variables|Default|SetgameInstance _asgame_instance_bp)
  (bind _asfp_sgame_mode_base (Utilities|Casting|CastToFpSGameModeBase (Game|GetGameMode)))
  (Variables|Default|SetgameMode _asfp_sgame_mode_base))

(fn LoadInfo
  (bind _asgame_instance_bp (Utilities|Casting|CastToGameInstanceBp (Variables|Default|GetgameInstance)))
  (Variables|Default|Sethealth (.Health (Utilities|Struct|BreakplayerInfo (Variables|/Game/Blueprints/GameInstanceBp.GameInstanceBp_C|GetplayerInfo _asgame_instance_bp))))
  (Variables|Default|Sethunger (.Hunger (Utilities|Struct|BreakplayerInfo (Variables|/Game/Blueprints/GameInstanceBp.GameInstanceBp_C|GetplayerInfo _asgame_instance_bp))))
  (Variables|Default|Setfood (.Food (Utilities|Struct|BreakplayerInfo (Variables|/Game/Blueprints/GameInstanceBp.GameInstanceBp_C|GetplayerInfo _asgame_instance_bp))))
  (Variables|Default|Setwood (.Wood (Utilities|Struct|BreakplayerInfo (Variables|/Game/Blueprints/GameInstanceBp.GameInstanceBp_C|GetplayerInfo _asgame_instance_bp))))
  (Variables|Default|Setstone (.Stone (Utilities|Struct|BreakplayerInfo (Variables|/Game/Blueprints/GameInstanceBp.GameInstanceBp_C|GetplayerInfo _asgame_instance_bp))))
  (Variables|Default|Setiron (.Irom (Utilities|Struct|BreakplayerInfo (Variables|/Game/Blueprints/GameInstanceBp.GameInstanceBp_C|GetplayerInfo _asgame_instance_bp))))
  (Variables|Default|Setcoins (.Coins (Utilities|Struct|BreakplayerInfo (Variables|/Game/Blueprints/GameInstanceBp.GameInstanceBp_C|GetplayerInfo _asgame_instance_bp)))))

(fn GameOver
  (bind _returnvalue (Game|SetGamePaused true))
  (if _returnvalue
    (Viewport|RemoveAllWidgets)
    (bind _returnvalue_2 (UserInterface|CreateWidget "/Game/UI/gameOverUi.gameOverUi_C"))
    (UserInterface|Viewport|AddtoViewport _returnvalue_2 0)))

(fn HasResource
  (params (cost :type Ent%20Cost%20Structure))
  (bind (_wood _stone _iron _food) (Utilities|Struct|BreakentCost cost))
  (Utilities|FlowControl|Sequence
    (:then_0
      (if (>= (Variables|Default|Getwood) _wood)
        (LocalVariables|Sethas? true)
        (else
          (LocalVariables|Sethas? false)
          (return (LocalVariables|Gethas?)))))
    (:then_1
      (if (>= (Variables|Default|Getstone) _stone)
        (LocalVariables|Sethas? true)
        (else
          (LocalVariables|Sethas? false)
          (return (LocalVariables|Gethas?)))))
    (:then_2
      (if (>= (Variables|Default|Getiron) _iron)
        (LocalVariables|Sethas? true)
        (else
          (LocalVariables|Sethas? false)
          (return (LocalVariables|Gethas?)))))
    (:then_3
      (if (>= (Variables|Default|Getfood) _food)
        (LocalVariables|Sethas? true)
        (else
          (LocalVariables|Sethas? false)
          (return (LocalVariables|Gethas?)))))
    (:then_4
      (return (LocalVariables|Gethas?)))))

(fn Dmg/min
  (params (dmg :type Float%20%28single-precision%29))
  (bind _returnvalue (Utilities|Time|GetWorldDeltaSeconds))
  (bind _dmgarray (Variables|Default|GetdmgArray))
  (bind _output_get (LocalVariables|SetcurTime _returnvalue))
  (if (== (Variables|Default|Getdmg) 0.0)
    (LocalVariables|SetstTime _returnvalue))
  (if (< (- (LocalVariables|GetstTime) _output_get) 6e+01)
    (Variables|Default|Setdmg (+ (Variables|Default|Getdmg) dmg))
    (else
      (Utilities|Array|Add _dmgarray (Variables|Default|Getdmg))
      (Variables|Default|Setdmg 0.0)
      (for _array_element _dmgarray
        (Variables|Default|SetdmgSum (+ (Variables|Default|GetdmgSum) _array_element)))
      (Utilities|Struct|SetmembersinscoreInfo (Variables|Default|Getscore) (/ (Math|Conversions|ToFloat(Integer) (Utilities|Array|Length _dmgarray)) (Variables|Default|GetdmgSum))))))

(fn Kls/mnt
  (bind _returnvalue (Utilities|Time|GetWorldDeltaSeconds))
  (bind _kills_minute (Variables|Default|Getkills/minute))
  (bind _output_get (LocalVariables|SetcurrTime _returnvalue))
  (if (== (Variables|Default|GetcurrentKills) 0)
    (LocalVariables|SetstrTime _returnvalue))
  (if (< (- _output_get (LocalVariables|GetstrTime)) 6e+01)
    (Variables|Default|SetcurrentKills (+ (Variables|Default|GetcurrentKills) 1))
    (else
      (Utilities|Array|Add _kills_minute (Variables|Default|GetcurrentKills))
      (Variables|Default|SetcurrentKills 0)
      (for _array_element _kills_minute
        (Variables|Default|SetkillsSum (+ (Variables|Default|GetkillsSum) _array_element)))
      (Utilities|Struct|SetmembersinscoreInfo (Variables|Default|Getscore) (/ (Math|Conversions|ToFloat(Integer) (Utilities|Array|Length _kills_minute)) (Math|Conversions|ToFloat(Integer) (Variables|Default|GetkillsSum)))))))

(fn CreateWidgets
  (bind _returnvalue (UserInterface|CreateWidget "/Game/UI/Settings.Settings_C"))
  (bind _output_get (Variables|Default|SetSettings _returnvalue))
  (UserInterface|Viewport|AddtoPlayerScreen _output_get))

(fn AndroidBack
  (bind _settings (Variables|Default|GetSettings))
  (bind _widgetswitcher_settings (Variables|/Game/UI/Settings.Settings_C|GetWidgetSwitcher_Settings _settings))
  (Utilities|FlowControl|Sequence
    (:then_0
      ;[1 1 1] Settings Close
      (if (> (Class|WidgetSwitcher|GetActiveWidgetIndex _widgetswitcher_settings) 0)
        (Class|WidgetSwitcher|SetActiveWidgetIndex _widgetswitcher_settings)
        (return)
        (elif (Widget|IsVisible _settings)
          (Widget|SetVisibility _settings "Hidden")
          (return))))
    (:then_1
      ;[1 1 1] Trap Overlay
      (bind _asfp_sgame_mode_base (Utilities|Casting|CastToFpSGameModeBase (Game|GetGameMode)))
      (if (Widget|IsVisible (Variables|/Game/UI/mainGameUi.mainGameUi_C|GettrapOverlay (Variables|/Game/Blueprints/FpSGameModeBase.FpSGameModeBase_C|GetMainGameUi _asfp_sgame_mode_base)))
        (Default|BackButtonTrap (Variables|/Game/Blueprints/FpSGameModeBase.FpSGameModeBase_C|GetMainGameUi _asfp_sgame_mode_base))
        (return)))
    (:then_2
      ;[1 1 1] Crafting Overlay
      (bind _asfp_sgame_mode_base_2 (Utilities|Casting|CastToFpSGameModeBase (Game|GetGameMode)))
      (if (Widget|IsVisible (Variables|/Game/UI/mainGameUi.mainGameUi_C|GetcraftingOverlay (Variables|/Game/Blueprints/FpSGameModeBase.FpSGameModeBase_C|GetMainGameUi _asfp_sgame_mode_base_2)))
        (Default|BackButtonCrafting (Variables|/Game/Blueprints/FpSGameModeBase.FpSGameModeBase_C|GetMainGameUi _asfp_sgame_mode_base_2))
        (return)))
    (:then_3
      ;[1 1 1] Settings Open
      (Widget|SetVisibility (Variables|Default|GetSettings) "Visible")
      (return))))