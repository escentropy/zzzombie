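; Animal pawn that wanders randomly and can be killed by clicking its static mesh.
; Tick feeds a random-length Delay, acting as a repeating timer that sends AIMoveTo to a random reachable point nearby and tracks IsMoving.
; Each click deals fixed damage through EntityDmg, then, if ChkDead reports death, calls UpdateRes and destroys the actor.
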(event OnClicked(StaticMesh)
  (params (TouchedComponent :type Primitive%20Component%20Object%20Reference) (ButtonPressed :type Key%20Structure :default "None"))
  (CallFunction|EntityDmg 25.0)
  (bind _isdead (CallFunction|ChkDead))
  (if _isdead
    (CallFunction|UpdateRes)
    (Actor|DestroyActor)))

(event EventBeginPlay
  (|CallParentFunction) ; This node is disabled and will not be called.\nDrag off pins to build functionality.
)

(event Collision|EventActorBeginOverlap
  (params (OtherActor :type Actor%20Object%20Reference))
  (|CallParentFunction OtherActor) ; This node is disabled and will not be called.\nDrag off pins to build functionality.
)

(event EventTick
  (params (DeltaSeconds :type Float%20%28single-precision%29))
  (|CallParentFunction DeltaSeconds)
  (Utilities|FlowControl|Delay (Math|Random|RandomFloatinRange 1.0 5.0))
  (Variables|Default|SetisMoving true)
  (AI|AIMoveTo self (.RandomLocation (AI|Navigation|GetRandomReachablePointinRadius (Transformation|GetActorLocation) 1e+03 0 0)) 0 5.0 false
    (:OnSuccess
      _)
    (:OnFail
      _))
  (Variables|Default|SetisMoving false))

(fn ConstructionScript
  (|CallParentFunction))