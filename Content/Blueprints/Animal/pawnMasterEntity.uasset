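; Base animal pawn that holds health and provides helpers for damage, death checks, food rewards and player stamina costs.
; On BeginPlay it registers itself as the owner of its life-progress widget.
; Helper functions reduce and test its Health, or cast to FpSPlayerController to add one Food and to check or spend Stamina.
; The mesh click event is empty, and nothing here calls the helpers.
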(event OnClicked(StaticMesh)
  (params (TouchedComponent :type Primitive%20Component%20Object%20Reference) (ButtonPressed :type Key%20Structure :default "None")))

(event EventBeginPlay
  (bind _aspawn_life_progress (Utilities|Casting|CastTopawnLifeProgress (UserInterface|GetUserWidgetObject (Variables|Default|GetWidget))))
  (Variables|/Game/UI/pawnLifeProgress.pawnLifeProgress_C|SetactorOwner _aspawn_life_progress self))

(event Collision|EventActorBeginOverlap
  (params (OtherActor :type Actor%20Object%20Reference)))

(event EventTick
  (params (DeltaSeconds :type Float%20%28single-precision%29)))

(fn ConstructionScript)

(fn EntityDmg
  (params (amount :type Float%20%28single-precision%29))
  (Variables|Default|Sethealth (- (Variables|Default|Gethealth) amount)))

(fn ChkDead
  (if (> (Variables|Default|Gethealth) 0.0)
    (LocalVariables|Setdead false)
    (else
      (LocalVariables|Setdead true)))
  (return (LocalVariables|Getdead)))

(fn UpdateRes
  (bind _asfp_splayer_controller (Utilities|Casting|CastToFpSPlayerController (Game|GetPlayerController 0)))
  (Variables|/Game/Blueprints/FpSPlayerController.FpSPlayerController_C|Setfood _asfp_splayer_controller (+ (Variables|/Game/Blueprints/FpSPlayerController.FpSPlayerController_C|Getfood _asfp_splayer_controller) 1)))

(fn ChkStmn
  (bind _asfp_splayer_controller (Utilities|Casting|CastToFpSPlayerController (Game|GetPlayerController 0)))
  (if (> (Variables|/Game/Blueprints/FpSPlayerController.FpSPlayerController_C|Getstamina _asfp_splayer_controller) 0.0)
    (LocalVariables|Setstamina? true)
    (else
      (LocalVariables|Setstamina? false)))
  (return (LocalVariables|Getstamina?)))

(fn DecStmn
  (params (amoount :type Float%20%28single-precision%29))
  (bind _asfp_splayer_controller (Utilities|Casting|CastToFpSPlayerController (Game|GetPlayerController 0)))
  (Variables|/Game/Blueprints/FpSPlayerController.FpSPlayerController_C|Setstamina _asfp_splayer_controller (- (Variables|/Game/Blueprints/FpSPlayerController.FpSPlayerController_C|Getstamina _asfp_splayer_controller) amoount)))