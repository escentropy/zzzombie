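; Inventory system Blueprint that tracks which tool or weapon occupies each type slot: axe, pickaxe, melee, range and hammer.
; SetItem writes the item's id into the ItemSlotIds index matching its type.
; GetItem uses that stored id to look up the item in the matching ToolManager array.
; GetEquipedItem separately returns the equipped Tool or Weapon from the two-entry EquipedTools array.
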(fn GetItem
  (params (typeSlot :type Integer))
  (bind _toolmanager (Variables|Default|GettoolManager))
  (bind _itemslotids (Variables|Default|GetitemSlotIds))
  (bind _output (Utilities|Array|Get(acopy) _itemslotids typeSlot))
  (switch int typeSlot
    (:0
      (LocalVariables|SetitemLc (Utilities|Array|Get(acopy) (Variables|/Game/Blueprints/Tools/ToolManagerBp.ToolManagerBp_C|Getaxes _toolmanager) _output)))
    (:1
      (LocalVariables|SetitemLc (Utilities|Array|Get(acopy) (Variables|/Game/Blueprints/Tools/ToolManagerBp.ToolManagerBp_C|Getpickaxes _toolmanager) _output)))
    (:2
      (LocalVariables|SetitemLc (Utilities|Array|Get(acopy) (Variables|/Game/Blueprints/Tools/ToolManagerBp.ToolManagerBp_C|Getmelees _toolmanager) _output)))
    (:3
      (LocalVariables|SetitemLc (Utilities|Array|Get(acopy) (Variables|/Game/Blueprints/Tools/ToolManagerBp.ToolManagerBp_C|Getranges _toolmanager) _output)))
    (:4
      (LocalVariables|SetitemLc (Utilities|Array|Get(acopy) (Variables|/Game/Blueprints/Tools/ToolManagerBp.ToolManagerBp_C|Gethammers _toolmanager) _output))))
  (return (LocalVariables|GetitemLc)))

(fn SetItem
  (params (item :type Tools%20Master%20Object%20Reference))
  (bind _itemslotids (Variables|Default|GetitemSlotIds))
  (bind _info (Variables|/Game/Blueprints/Tools/ToolsMaster.ToolsMaster_C|Getinfo item))
  (switch Utilities|FlowControl|Switch|SwitchontypeToolEnum (.type _info)
    (:NewEnumerator0
      (Utilities|Array|SetArrayElem _itemslotids 0 (.id _info)))
    (:NewEnumerator1
      (Utilities|Array|SetArrayElem _itemslotids 1 (.id _info)))
    (:NewEnumerator2
      (Utilities|Array|SetArrayElem _itemslotids 2 (.id _info)))
    (:NewEnumerator3
      (Utilities|Array|SetArrayElem _itemslotids 3 (.id _info)))
    (:NewEnumerator4
      (Utilities|Array|SetArrayElem _itemslotids 4 (.id _info)))))

(fn GetEquipedItem
  (params (type :type newTypeEnum%20Enum :default "NewEnumerator5"))
  (bind _equipedtools (Variables|Default|GetequipedTools))
  (switch Utilities|FlowControl|Switch|SwitchonnewTypeEnum type
    (:NewEnumerator5
      (LocalVariables|SetitemLc (Utilities|Array|Get(acopy) _equipedtools)))
    (:NewEnumerator6
      (LocalVariables|SetitemLc (Utilities|Array|Get(acopy) _equipedtools 1))))
  (return (LocalVariables|GetitemLc)))