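; Clickable stone resource entity that the player damages at a stamina cost to gain resources.
; A click on its static mesh checks stamina, then spends a fixed amount and damages the entity.
; If the entity is then dead, it calls UpdateRes to update resources.
; The stamina, damage, death and resource functions are called here but defined outside this graph, and the default events are unused.
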(event OnClicked(StaticMesh)
  (params (TouchedComponent :type Primitive%20Component%20Object%20Reference) (ButtonPressed :type Key%20Structure :default "None"))
  (bind _hasstamina (CallFunction|ChkStamina))
  (if _hasstamina
    (CallFunction|DecStamina 35.0)
    (CallFunction|EntityDmg 2.0)
    (bind _isdead (CallFunction|ChkDead))
    (if _isdead
      (CallFunction|UpdateRes 1))))

(event EventBeginPlay
  (|CallParentFunction) ; This node is disabled and will not be called.\nDrag off pins to build functionality.
)

(event Collision|EventActorBeginOverlap
  (params (OtherActor :type Actor%20Object%20Reference))
  (|CallParentFunction OtherActor) ; This node is disabled and will not be called.\nDrag off pins to build functionality.
)

(event EventTick
  (params (DeltaSeconds :type Float%20%28single-precision%29))
  (|CallParentFunction DeltaSeconds) ; This node is disabled and will not be called.\nDrag off pins to build functionality.
)

(fn ConstructionScript
  (|CallParentFunction))