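; Base actor for clickable, harvestable entities such as trees, which grant resources to the player.
; Each mesh click deals one damage to Health and adds one Wood through FpSPlayerController.
; BeginPlay hands the actor to its life-progress widget, while Tick polls Health and destroys the actor once depleted.
; Helpers also support Stone rewards and stamina checks or costs, though the event graph never uses them.
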(event OnClicked(StaticMesh)
  (params (TouchedComponent :type Primitive%20Component%20Object%20Reference) (ButtonPressed :type Key%20Structure :default "None"))
  (CallFunction|EntityDmg 1.0)
  (CallFunction|UpdateRes))

(event EventBeginPlay
  (bind _asactor_life_progress (Utilities|Casting|CastToactorLifeProgress (UserInterface|GetUserWidgetObject (Variables|Default|GetWidget))))
  (Variables|/Game/UI/actorLifeProgress.actorLifeProgress_C|SetactorOwner _asactor_life_progress self))

(event Collision|EventActorBeginOverlap
  (params (OtherActor :type Actor%20Object%20Reference)))

(event EventTick
  (params (DeltaSeconds :type Float%20%28single-precision%29))
  (bind _isdead (CallFunction|ChkDead))
  (if _isdead
    (Actor|DestroyActor)))

(fn ConstructionScript)

(fn EntityDmg
  (params (amount :type Float%20%28single-precision%29))
  (Variables|Default|Sethealth (- (Variables|Default|Gethealth) amount)))

(fn ChkDead
  (if (> (Variables|Default|Gethealth) 0.0)
    (LocalVariables|Setdead false)
    (else
      (LocalVariables|Setdead true)))
  (return (LocalVariables|Getdead)))

(fn UpdateRes
  (params (entId :type Integer))
  (bind _asfp_splayer_controller (Utilities|Casting|CastToFpSPlayerController (Game|GetPlayerController 0)))
  (switch int entId
    (:0
      (Variables|/Game/Blueprints/FpSPlayerController.FpSPlayerController_C|Setwood _asfp_splayer_controller (+ (Variables|/Game/Blueprints/FpSPlayerController.FpSPlayerController_C|Getwood _asfp_splayer_controller) 1)))
    (:1
      (Variables|/Game/Blueprints/FpSPlayerController.FpSPlayerController_C|Setstone _asfp_splayer_controller (+ (Variables|/Game/Blueprints/FpSPlayerController.FpSPlayerController_C|Getstone _asfp_splayer_controller) 1)))))

(fn DecStamina
  (params (amount :type Float%20%28single-precision%29))
  (bind _asfp_splayer_controller (Utilities|Casting|CastToFpSPlayerController (Game|GetPlayerController 0)))
  (Variables|/Game/Blueprints/FpSPlayerController.FpSPlayerController_C|Setstamina _asfp_splayer_controller (- (Variables|/Game/Blueprints/FpSPlayerController.FpSPlayerController_C|Getstamina _asfp_splayer_controller) amount)))

(fn ChkStamina
  (bind _asfp_splayer_controller (Utilities|Casting|CastToFpSPlayerController (Game|GetPlayerController 0)))
  (if (> (Variables|/Game/Blueprints/FpSPlayerController.FpSPlayerController_C|Getstamina _asfp_splayer_controller) 0.0)
    (LocalVariables|Setstamina? true)
    (else
      (LocalVariables|Setstamina? false)))
  (return (LocalVariables|Getstamina?)))