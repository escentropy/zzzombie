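; Doctor zombie boss that heals other zombies around it.
; BeginPlay attaches a stethoscope, head mirror and syringe to mesh sockets and, outside the editor flag, switches to the boss soundtrack and marks itself as boss.
; A Delay on Tick paces the heal to about once a second, topping up health of zombies overlapping AbilityArea to a cap.
; When IsDead is set, Tick destroys the props and calls BossIsDead.
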(event Custom|ability
  ;[1 1 1] ability
  (for _array_element (Collision|GetOverlappingActors (Variables|Default|GetabilityArea) "/Game/Blueprints/enemy/enemyZombie.enemyZombie_C" :!class /Script/Engine.PrimitiveComponent)
    (bind _asenemy_zombie (Utilities|Casting|CastToenemyZombie _array_element))
    (if (!= _asenemy_zombie self)
      (if (> (+ (Variables|/Game/Blueprints/Resources/entityMasterBp.entityMasterBp_C|GetconstHealth _asenemy_zombie) 25.0) 1e+02)
        (Variables|/Game/Blueprints/Resources/entityMasterBp.entityMasterBp_C|SetconstHealth _asenemy_zombie 1e+02)
        (else
          (Variables|/Game/Blueprints/Resources/entityMasterBp.entityMasterBp_C|SetconstHealth _asenemy_zombie (+ (Variables|/Game/Blueprints/Resources/entityMasterBp.entityMasterBp_C|GetconstHealth _asenemy_zombie) 25.0)))))))

(event EventBeginPlay
  (|CallParentFunction)
  (CallFunction|GetRandomMaterial)
  ;[1 1 1] Equip Stethoscope
  (bind _returnvalue (Game|SpawnActorfromClass "/Game/Zombie/Zombie_boss_06/Equipments/Stethoscope_bp.Stethoscope_bp_C" (Transformation|GetActorTransform) "Undefined" 0 0))
  (bind _output_get (Variables|Default|Setscope _returnvalue))
  (Transformation|AttachComponentToComponent _returnvalue (Variables|Default|GetSkeletalMesh) "HeadSocket2" "SnapToTarget" "SnapToTarget" "SnapToTarget" true)
  ;[1 1 1] Equip Headmirror
  (bind _returnvalue_2 (Game|SpawnActorfromClass "/Game/Zombie/Zombie_boss_06/Equipments/HeadMirror_bp.HeadMirror_bp_C" (Transformation|GetActorTransform) "Undefined" 0 0))
  (bind _output_get_2 (Variables|Default|SetheadMirror _returnvalue_2))
  (Transformation|AttachComponentToComponent _output_get_2 (Variables|Default|GetSkeletalMesh) "HeadSocket" "SnapToTarget" "SnapToTarget" "SnapToTarget" true)
  ;[1 1 1] Equip Weapon
  (bind _returnvalue_3 (Game|SpawnActorfromClass "/Game/Zombie/Zombie_boss_06/Equipments/Syrigne_bp.Syrigne_bp_C" (Transformation|GetActorTransform) "Undefined" 0 0))
  (bind _output_get_3 (Variables|Default|Setsyringe _returnvalue_3))
  (Transformation|AttachComponentToComponent _output_get_3 (Variables|Default|GetSkeletalMesh) "Hand_socket" "SnapToTarget" "SnapToTarget" "SnapToTarget" true)
  (if (not (Variables|Default|Geteditor_0))
    (CallFunction|ChangeSoundtrack)
    (Variables|Default|SetIsBoss? true)))

(event Collision|EventActorBeginOverlap
  (params (OtherActor :type Actor%20Object%20Reference))
  (|CallParentFunction OtherActor) ; This node is disabled and will not be called.\nDrag off pins to build functionality.
)

(event EventTick
  (params (DeltaSeconds :type Float%20%28single-precision%29))
  (bind _scope (Variables|Default|Getscope))
  (bind _headmirror (Variables|Default|GetheadMirror))
  (bind _syringe (Variables|Default|Getsyringe))
  ;[1 1 1] tick
  (|CallParentFunction DeltaSeconds)
  (Utilities|FlowControl|Sequence
    (:then_0
      (Utilities|FlowControl|Delay 1.0)
      (CallFunction|Ability))
    (:then_1
      (if (Variables|Default|GetisDead)
        (Utilities|FlowControl|Sequence
          (:then_0
            (if (Utilities|IsValid _scope)
              (Actor|DestroyActor _scope)))
          (:then_1
            (if (Utilities|IsValid _headmirror)
              (Actor|DestroyActor _headmirror)))
          (:then_2
            (if (Utilities|IsValid _syringe)
              (Actor|DestroyActor _syringe)))
          (:then_3
            (CallFunction|BossIsDead)))))))

(fn ConstructionScript
  (|CallParentFunction)
  (Variables|Default|SetSpecialSoundtrack "/Game/Sounds/SoundtrackParts/Part_2_Boss_1___main_funk__Cue.Part_2_Boss_1___main_funk__Cue"))