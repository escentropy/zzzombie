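; Final necromancer zombie boss that summons other bosses and teleports between tiles, with its own soundtrack.
; BeginPlay attaches a beard and scepter to skeletal sockets; both are destroyed on death.
; Tick halts and reveals it below an X threshold, then Ability spawns a random GameMode boss if SpawnArea is clear.
; It then hides and retries random tiles on a delay, though the occupancy check and move roll separate indices.
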(event Custom|Ability
  (bind _tiles (Variables|Default|Gettiles))
  (bind _returnvalue (Utilities|Array|Length _tiles))
  (bind _returnvalue_2 (Math|Random|RandomIntegerinRange 14 _returnvalue))
  (bind _output (Utilities|Array|Get(acopy) _tiles _returnvalue_2))
  ;[1 1 1] Ability
  (if (== (Utilities|Array|Length (Collision|GetOverlappingActors (Variables|Default|GetspawnArea) "/Game/Blueprints/Resources/entityMasterBp.entityMasterBp_C" :!class /Script/Engine.PrimitiveComponent)) 0)
    (Game|SpawnActorfromClass (Utilities|GetClass (Utilities|Array|Get(acopy) (Variables|/Game/Blueprints/FpSGameModeBase.FpSGameModeBase_C|GetbossActors (Variables|Default|GetgameMode)) (Math|Random|RandomIntegerinRange 0 3))) (Math|Conversions|ToTransform(Vector) (Transformation|GetWorldLocation (Variables|Default|GetspawnVecor))) "Undefined" 0 0))
  (Utilities|FlowControl|Delay 5.0)
  (CallFunction|HideBoss :!label _label)
  (if (Variables|/Game/Blueprints/TileSystem/tilesBp.tilesBp_C|Getoccupied _output)
    (Utilities|FlowControl|Delay 2.0)
    (goto _label)
    (else
      (Transformation|SetWorldLocation (Variables|Default|GetBox) (Transformation|GetWorldLocation (Variables|/Game/Blueprints/TileSystem/tilesBp.tilesBp_C|GetspawnVector _output)) false false)
      (Utilities|FlowControl|Delay 5.0)
      (Variables|Default|SetabilityReady false)
      (Rendering|SetActorHiddenInGame self true))))

(event EventBeginPlay
  (|CallParentFunction)
  (bind _outactors (Actor|GetAllActorsOfClass "/Game/Blueprints/TileSystem/tilesBp.tilesBp_C"))
  (Variables|Default|Settiles _outactors)
  (CallFunction|GetRandomMaterial)
  ;[1 1 1] Equip beard
  (bind _returnvalue (Game|SpawnActorfromClass "/Game/Zombie/Zombie_boss_05/Equipment/beard_bp.beard_bp_C" (Transformation|GetActorTransform) "Undefined" 0 0))
  (Variables|Default|SetBeard _returnvalue)
  (Transformation|AttachComponentToComponent _returnvalue (Variables|Default|GetSkeletalMesh) "Bip001-HeadNubSocket" "SnapToTarget" "SnapToTarget" "SnapToTarget" true)
  ;[1 1 1] Equip beard
  (bind _returnvalue_2 (Game|SpawnActorfromClass "/Game/Zombie/Zombie_boss_05/Equipment/Scypter_bp.Scypter_bp_C" (Transformation|GetActorTransform) "Undefined" 0 0))
  (bind _output_get (Variables|Default|SetScypter _returnvalue_2))
  (Transformation|AttachComponentToComponent _output_get (Variables|Default|GetSkeletalMesh) "Bip001-R-Finger0NubSocket" "SnapToTarget" "SnapToTarget" "SnapToTarget" true)
  (if (not (Variables|Default|Geteditor_0))
    (CallFunction|ChangeSoundtrack)
    (Variables|Default|SetIsBoss? true)))

(event Collision|EventActorBeginOverlap
  (params (OtherActor :type Actor%20Object%20Reference))
  (|CallParentFunction OtherActor) ; This node is disabled and will not be called.\nDrag off pins to build functionality.
)

(event EventTick
  (params (DeltaSeconds :type Float%20%28single-precision%29))
  ;[1 1 1] Tick
  (if (not (Variables|Default|Geteditor_0))
    (|CallParentFunction DeltaSeconds)
    (if (Variables|Default|GetisDead)
      (Utilities|FlowControl|DoOnce false
        (:Completed
          (Actor|DestroyActor (Variables|Default|GetBeard))
          (Actor|DestroyActor (Variables|Default|GetScypter))))
      (else
        (Utilities|FlowControl|Sequence
          (:then_0
            (if (< (.x (Transformation|GetWorldLocation (Variables|Default|GetBox))) 1.3e+03)
              (if (Variables|Default|GetabilityReady)
                (Utilities|FlowControl|DoOnce false :!label _label
                  (:Completed
                    (CallFunction|ShowBoss)
                    (Variables|Default|SetmoveSpeed 0.0)
                    (Utilities|Struct|SetmembersinenemyStatsStr (Variables|Default|GetStats) 0.0)
                    (Utilities|FlowControl|Delay 5.0)
                    (CallFunction|Ability)))
                (else
                  (Utilities|FlowControl|Sequence
                    (:then_0
                      (goto _label Reset))
                    (:then_1
                      (Variables|Default|SetabilityReady true))))))))))))

(fn ConstructionScript
  (|CallParentFunction)
  (Variables|Default|SetSpecialSoundtrack "/Game/Sounds/SoundtrackParts/NecroMASTER_2_Cue.NecroMASTER_2_Cue"))

(fn HideBoss
  (Rendering|SetActorHiddenInGame true)
  (Rendering|SetActorHiddenInGame (Variables|Default|GetBeard) true)
  (Rendering|SetActorHiddenInGame (Variables|Default|GetScypter) true)
  (Collision|SetCollisionEnabled (Variables|Default|GettouchCollision) "NoCollision"))

(fn ShowBoss
  (Rendering|SetActorHiddenInGame false)
  (Rendering|SetActorHiddenInGame (Variables|Default|GetBeard) false)
  (Rendering|SetActorHiddenInGame (Variables|Default|GetScypter) false)
  (Collision|SetCollisionEnabled (Variables|Default|GetBox) "QueryOnly"))