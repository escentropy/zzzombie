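; Armored zombie boss that spawns socket-attached helmet, armor and shield and switches to boss music.
; Tick marches it along local X, damaging the player and removing it past a threshold, or handles death.
; Clicks or touches deal weapon damage, firing ammunition for ranged hits; falling health sheds gear in stages, then adds blood bursts and stagger.
; Its Blocking component makes overlapping zombies invulnerable; boss removal restores damageability to all.
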(event OnClicked(StaticMesh1)
  (params (TouchedComponent :type Primitive%20Component%20Object%20Reference) (ButtonPressed :type Key%20Structure :default "None"))
  (bind _returnvalue (Transformation|GetActorTransform))
  (bind _shield (Variables|Default|Getshield))
  (bind _box (Variables|Default|GetBox))
  (bind _armor (Variables|Default|Getarmor))
  (bind _consthealth (Variables|Default|GetconstHealth))
  (bind _helmet (Variables|Default|Gethelmet))
  (bind _returnvalue_2 (Transformation|GetWorldLocation _box))
  ;[1 1 1] onClick
  (if (not (Variables|Default|GetisDead))
    (bind (_weapontype _hit_) (CallFunction|GetItemDistance))
    (if _hit_
      (CallFunction|RapidClick (Utilities|Time|GetTimeSeconds))
      (if (Variables|Default|Getrange?)
        (if (Variables|/Game/Blueprints/DebugModeBp.DebugModeBp_C|Getdebug? (Variables|Default|GetdebugMode))
          (bind _returnvalue_3 (Game|SpawnActorfromClass "/Game/Blueprints/ammunitionBp.ammunitionBp_C" (Math|Transform|MakeTransform (Math|Vector|MakeVector 3.4e+02 (.y _returnvalue_2) 0.0) "0, 0, 0" "1,1,1") "Undefined" 0 0 :!label _label))
          (Variables|/Game/Blueprints/ammunitionBp.ammunitionBp_C|Settarget _returnvalue_3 (Math|Vector|MakeVector (.x _returnvalue_2) 0.0 0.0))
          (CallFunction|EntityDmg (.dmg (Variables|/Game/Blueprints/Tools/ToolsMaster.ToolsMaster_C|Getinfo _weapontype)) (.Health (Utilities|Struct|BreakenemyStatsStr (Variables|Default|GetStats))) :!label _label_2)
          (if (< _consthealth 3e+01)
            (bind _returnvalue_4 (Effects|SpawnEmitteratLocation "/Game/Particles/P_Bloodburst.P_Bloodburst" (Math|Vector|MakeVector (+ (.x (.location _returnvalue)) 1e+02) (.y (.location _returnvalue)) (.z (.location _returnvalue))) "0, 0, 0" "1.000000,1.000000,1.000000" false "None" false))
            (bind _output_get (Variables|Default|SetBloodBurstEmitter _returnvalue_4))
            (Components|Activation|Activate _output_get true)
            (Variables|Default|SetmoveSpeed 0.0)
            (Utilities|FlowControl|Delay 0.2)
            (Utilities|FlowControl|Delay 0.8)
            (Variables|Default|Setattacked? false)
            (Variables|Default|SetmoveSpeed (.Speed (Utilities|Struct|BreakenemyStatsStr (Variables|Default|GetStats))))
            (else
              (Utilities|FlowControl|Sequence
                (:then_0
                  (if (< _consthealth 8e+01)
                    (Utilities|FlowControl|DoOnce false
                      (:Completed
                        (Transformation|DetachFromActor _helmet "KeepRelative" "KeepRelative" "KeepRelative")
                        (Actor|DestroyActor _helmet)))))
                (:then_1
                  (if (< _consthealth 6e+01)
                    (Utilities|FlowControl|DoOnce false
                      (:Completed
                        (Transformation|DetachFromActor _armor "KeepRelative" "KeepRelative" "KeepRelative")
                        (Actor|DestroyActor _armor)))))
                (:then_2
                  (if (< _consthealth 4e+01)
                    (Utilities|FlowControl|DoOnce false
                      (:Completed
                        (Transformation|DetachFromActor _shield "KeepRelative" "KeepRelative" "KeepRelative")
                        (Actor|DestroyActor _shield))))))))
          (else
            (bind _hasammun (CallFunction|CheckAmmunition (.id (Variables|/Game/Blueprints/Tools/ToolsMaster.ToolsMaster_C|Getinfo _weapontype))))
            (if _hasammun
              (goto _label))))
        (else
          (goto _label_2))))))

(event OnInputTouchBegin(StaticMesh1)
  (params (FingerIndex :type ETouchIndex%20Enum :default "Touch1") (TouchedComponent :type Primitive%20Component%20Object%20Reference))
  (bind _returnvalue (Transformation|GetActorTransform))
  (bind _shield (Variables|Default|Getshield))
  (bind _box (Variables|Default|GetBox))
  (bind _armor (Variables|Default|Getarmor))
  (bind _consthealth (Variables|Default|GetconstHealth))
  (bind _helmet (Variables|Default|Gethelmet))
  (bind _returnvalue_2 (Transformation|GetWorldLocation _box))
  ;[1 1 1] onClick
  (if (not (Variables|Default|GetisDead))
    (bind (_weapontype _hit_) (CallFunction|GetItemDistance))
    (if _hit_
      (CallFunction|RapidClick (Utilities|Time|GetTimeSeconds))
      (if (Variables|Default|Getrange?)
        (if (Variables|/Game/Blueprints/DebugModeBp.DebugModeBp_C|Getdebug? (Variables|Default|GetdebugMode))
          (bind _returnvalue_3 (Game|SpawnActorfromClass "/Game/Blueprints/ammunitionBp.ammunitionBp_C" (Math|Transform|MakeTransform (Math|Vector|MakeVector 3.4e+02 (.y _returnvalue_2) 0.0) "0, 0, 0" "1,1,1") "Undefined" 0 0 :!label _label))
          (Variables|/Game/Blueprints/ammunitionBp.ammunitionBp_C|Settarget _returnvalue_3 (Math|Vector|MakeVector (.x _returnvalue_2) 0.0 0.0))
          (CallFunction|EntityDmg (.dmg (Variables|/Game/Blueprints/Tools/ToolsMaster.ToolsMaster_C|Getinfo _weapontype)) (.Health (Utilities|Struct|BreakenemyStatsStr (Variables|Default|GetStats))) :!label _label_2)
          (if (< _consthealth 3e+01)
            (bind _returnvalue_4 (Effects|SpawnEmitteratLocation "/Game/Particles/P_Bloodburst.P_Bloodburst" (Math|Vector|MakeVector (+ (.x (.location _returnvalue)) 1e+02) (.y (.location _returnvalue)) (.z (.location _returnvalue))) "0, 0, 0" "1.000000,1.000000,1.000000" false "None" false))
            (bind _output_get (Variables|Default|SetBloodBurstEmitter _returnvalue_4))
            (Components|Activation|Activate _output_get true)
            (Variables|Default|SetmoveSpeed 0.0)
            (Utilities|FlowControl|Delay 0.2)
            (Utilities|FlowControl|Delay 0.8)
            (Variables|Default|Setattacked? false)
            (Variables|Default|SetmoveSpeed (.Speed (Utilities|Struct|BreakenemyStatsStr (Variables|Default|GetStats))))
            (else
              (Utilities|FlowControl|Sequence
                (:then_0
                  (if (< _consthealth 8e+01)
                    (Utilities|FlowControl|DoOnce false
                      (:Completed
                        (Transformation|DetachFromActor _helmet "KeepRelative" "KeepRelative" "KeepRelative")
                        (Actor|DestroyActor _helmet)))))
                (:then_1
                  (if (< _consthealth 6e+01)
                    (Utilities|FlowControl|DoOnce false
                      (:Completed
                        (Transformation|DetachFromActor _armor "KeepRelative" "KeepRelative" "KeepRelative")
                        (Actor|DestroyActor _armor)))))
                (:then_2
                  (if (< _consthealth 4e+01)
                    (Utilities|FlowControl|DoOnce false
                      (:Completed
                        (Transformation|DetachFromActor _shield "KeepRelative" "KeepRelative" "KeepRelative")
                        (Actor|DestroyActor _shield))))))))
          (else
            (bind _hasammun (CallFunction|CheckAmmunition (.id (Variables|/Game/Blueprints/Tools/ToolsMaster.ToolsMaster_C|Getinfo _weapontype))))
            (if _hasammun
              (goto _label))))
        (else
          (goto _label_2))))))

(event OnComponentBeginOverlap(blocking)
  (params (OverlappedComponent :type Primitive%20Component%20Object%20Reference) (OtherActor :type Actor%20Object%20Reference) (OtherComp :type Primitive%20Component%20Object%20Reference) (OtherBodyIndex :type Integer) (bFromSweep :type Boolean) (SweepResult :type Hit%20Result%20Structure%20%28by%20ref%29))
  (bind _asenemy_zombie (Utilities|Casting|CastToenemyZombie OtherActor))
  (for _array_element (Collision|GetOverlappingActors (Variables|Components|Getblocking) (Utilities|GetClass _asenemy_zombie) :!class /Script/Engine.PrimitiveComponent)
    (bind _asenemy_zombie_2 (Utilities|Casting|CastToenemyZombie _array_element))
    (Variables|/Game/Blueprints/enemy/enemyZombie.enemyZombie_C|SetcanBeDamaged _asenemy_zombie_2 false)))

(event OnComponentHit(blocking)
  (params (HitComponent :type Primitive%20Component%20Object%20Reference) (OtherActor :type Actor%20Object%20Reference) (OtherComp :type Primitive%20Component%20Object%20Reference) (NormalImpulse :type Vector :default "0, 0, 0") (Hit :type Hit%20Result%20Structure%20%28by%20ref%29))
  (bind _asenemy_zombie (Utilities|Casting|CastToenemyZombie OtherActor))
  (if (< (Utilities|Array|Length (Collision|GetOverlappingActors (Variables|Components|Getblocking) (Utilities|GetClass _asenemy_zombie) :!class /Script/Engine.PrimitiveComponent)) 1)
    (bind _outactors (Actor|GetAllActorsOfClass "/Game/Blueprints/enemy/enemyZombie.enemyZombie_C"))
    (for _array_element _outactors
      (bind _asenemy_zombie_2 (Utilities|Casting|CastToenemyZombie _array_element))
      (Variables|/Game/Blueprints/enemy/enemyZombie.enemyZombie_C|SetcanBeDamaged _asenemy_zombie_2 true))))

(event EventBeginPlay
  (|CallParentFunction)
  (CallFunction|GetRandomMaterial)
  ;[1 1 1] Equip Helmet
  (bind _returnvalue (Game|SpawnActorfromClass "/Game/Zombie/Zombie_boss_04/Equipments/RustyHelmet_BP.RustyHelmet_BP_C" (Transformation|GetActorTransform) "Undefined" 0 0))
  (bind _output_get (Variables|Default|Sethelmet _returnvalue))
  (Transformation|AttachComponentToComponent _output_get (Variables|Default|GetSkeletalMesh) "Bip001-HeadSocket" "SnapToTarget" "SnapToTarget" "SnapToTarget" true)
  ;[1 1 1] Equip Armor
  (bind _returnvalue_2 (Game|SpawnActorfromClass "/Game/Zombie/Zombie_boss_04/Equipments/RustyArmor_BP.RustyArmor_BP_C" (Transformation|GetActorTransform) "Undefined" 0 0))
  (bind _output_get_2 (Variables|Default|Setarmor _returnvalue_2))
  (Transformation|AttachComponentToComponent _output_get_2 (Variables|Default|GetSkeletalMesh) "Bip001-Spine2Socket" "SnapToTarget" "SnapToTarget" "SnapToTarget" true)
  ;[1 1 1] Equip Shield
  (bind _returnvalue_3 (Game|SpawnActorfromClass "/Game/Zombie/Zombie_boss_04/Equipments/RustyShield_BP.RustyShield_BP_C" (Transformation|GetActorTransform) "Undefined" 0 0))
  (bind _output_get_3 (Variables|Default|Setshield _returnvalue_3))
  (Collision|SetActorEnableCollision _output_get_3 false)
  (Transformation|AttachComponentToComponent _output_get_3 (Variables|Default|GetSkeletalMesh) "Bip001-R-Finger0NubSocket" "SnapToTarget" "SnapToTarget" "SnapToTarget" true)
  (if (not (Variables|Default|Geteditor_0))
    (CallFunction|ChangeSoundtrack)
    (Variables|Default|SetIsBoss? true)))

(event Collision|EventActorBeginOverlap
  (params (OtherActor :type Actor%20Object%20Reference))
  (|CallParentFunction OtherActor) ; This node is disabled and will not be called.\nDrag off pins to build functionality.
)

(event EventTick
  (params (DeltaSeconds :type Float%20%28single-precision%29))
  (bind _self self)
  ;[1 1 1] Tick
  (if (Utilities|IsValid _self)
    (bind _isdead (CallFunction|ChkDead))
    (if _isdead
      (bind _outactors (Actor|GetAllActorsOfClass "/Game/Blueprints/enemy/enemyZombie.enemyZombie_C"))
      (for _array_element _outactors
        (Variables|/Game/Blueprints/enemy/enemyZombie.enemyZombie_C|SetcanBeDamaged _array_element true)
        (Variables|Default|SetisDead true)
        (Utilities|FlowControl|Delay 2.0)
        (CallFunction|BossIsDead)
        (Actor|DestroyActor))
      (else
        (Class|Actor|AddActorLocalTransform (Math|Transform|MakeTransform (Math|Vector|MakeVector (Variables|Default|GetmoveSpeed) 0.0 0.0) "0, 0, 0" "1,1,1") false false)
        (if (< (.x (Transformation|GetActorLocation _self)) -3.7e+02)
          (Utilities|FlowControl|DoOnce false
            (:Completed
              (bind _asfp_splayer_controller (Utilities|Casting|CastToFpSPlayerController (Game|GetPlayerController 0)))
              (Variables|/Game/Blueprints/FpSPlayerController.FpSPlayerController_C|Sethealth _asfp_splayer_controller (- (Variables|/Game/Blueprints/FpSPlayerController.FpSPlayerController_C|Gethealth _asfp_splayer_controller) (.AttackHero (Utilities|Struct|BreakenemyStatsStr (Variables|Default|GetStats)))))
              (bind _outactors_2 (Actor|GetAllActorsOfClass "/Game/Blueprints/enemy/enemyZombie.enemyZombie_C"))
              (for _array_element_2 _outactors_2
                (Variables|/Game/Blueprints/enemy/enemyZombie.enemyZombie_C|SetcanBeDamaged _array_element_2 true))
              (Actor|DestroyActor (Variables|Default|Gethelmet))
              (Actor|DestroyActor (Variables|Default|Getarmor))
              (Actor|DestroyActor (Variables|Default|Getshield))
              (CallFunction|BossIsDead)
              (Actor|DestroyActor))))))))

(fn ConstructionScript
  (|CallParentFunction)
  (Variables|Default|SetSpecialSoundtrack "/Game/Sounds/SoundtrackParts/part_6_boss_3_Cue.part_6_boss_3_Cue"))