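; Female zombie enemy Blueprint that varies its appearance when it spawns and leaves other behavior to its parent class.
; On BeginPlay it runs the parent logic, calls GetRandomMaterial, then spawns a Hair_bp actor and snaps it to the head nub socket on the skeletal mesh.
; Tick and overlap events are disabled stubs, and the construction script only calls the parent.
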(event EventBeginPlay
  (|CallParentFunction)
  (CallFunction|GetRandomMaterial)
  ;[1 1 1] Equip hair
  (bind _returnvalue (Game|SpawnActorfromClass "/Game/Zombie/Zombie_01f/Equipment/hair_bp.hair_bp_C" (Transformation|GetActorTransform) "Undefined" 0 0))
  (Transformation|AttachComponentToComponent _returnvalue (Variables|Default|GetSkeletalMesh) "Bip001-HeadNubSocket" "SnapToTarget" "SnapToTarget" "SnapToTarget" true))

(event Collision|EventActorBeginOverlap
  (params (OtherActor :type Actor%20Object%20Reference))
  (|CallParentFunction OtherActor) ; This node is disabled and will not be called.\nDrag off pins to build functionality.
)

(event EventTick
  (params (DeltaSeconds :type Float%20%28single-precision%29))
  (|CallParentFunction DeltaSeconds) ; This node is disabled and will not be called.\nDrag off pins to build functionality.
)

(fn ConstructionScript
  (|CallParentFunction))