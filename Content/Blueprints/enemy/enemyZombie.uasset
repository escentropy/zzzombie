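; Zombie enemy with a random skin that advances each tick and, past a set X boundary, damages player health and destroys itself.
; Clicking it checks melee/range marker positions against the equipped weapon, spending resources as ranged ammo outside debug mode, then applies damage, blood and a brief stop.
; Box overlaps read component tags on entityMasterBp actors: obstacles halt movement, hittable entities take repeated timed attacks, and traps damage the zombie before being destroyed.
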(event OnClicked(StaticMesh)
  (params (TouchedComponent :type Primitive%20Component%20Object%20Reference) (ButtonPressed :type Key%20Structure :default "None"))
  (bind _returnvalue (Transformation|GetActorTransform))
  ;[1 1 1] OnClicked
  (bind (_weapontype _hit_) (CallFunction|GetItemDistance))
  (if _hit_
    (if (Variables|Default|Getrange?)
      (if (Variables|/Game/Blueprints/DebugModeBp.DebugModeBp_C|Getdebug? (Variables|Default|GetdebugMode))
        (CallFunction|EntityDmg (Math|Conversions|ToFloat(Integer) (.dmg (Variables|/Game/Blueprints/Tools/ToolsMaster.ToolsMaster_C|Getinfo _weapontype))) (Utilities|Struct|BreakenemyStatsStr (Variables|Default|GetStats)) :!label _label)
        (Variables|Default|Setattacked? true)
        (bind _returnvalue_2 (Effects|SpawnEmitteratLocation "/Game/Particles/Blood_Burst/P_Bloodburst.P_Bloodburst" (Math|Vector|MakeVector (+ (.x (.location _returnvalue)) 1e+02) (.y (.location _returnvalue)) (.z (.location _returnvalue))) "0, 0, 0" "1.000000,1.000000,1.000000" false "None" false))
        (bind _output_get (Variables|Default|SetBloodBurstEmitter _returnvalue_2))
        (Components|Activation|Activate _output_get true)
        (Variables|Default|SetmoveSpeed 0.0)
        (Utilities|FlowControl|Delay 0.2)
        (Components|Activation|Deactivate _output_get)
        (Components|DestroyComponent (Variables|Default|GetBloodBurstEmitter))
        (Utilities|FlowControl|Delay 0.8)
        (Variables|Default|Setattacked? false)
        (Variables|Default|SetmoveSpeed (Utilities|Struct|BreakenemyStatsStr (Variables|Default|GetStats)))
        (else
          (bind _hasammun (CallFunction|CheckAmmunition (.id (Variables|/Game/Blueprints/Tools/ToolsMaster.ToolsMaster_C|Getinfo _weapontype))))
          (if _hasammun
            (goto _label))))
      (else
        (goto _label)))))

(event OnComponentBeginOverlap(Box)
  (params (OverlappedComponent :type Primitive%20Component%20Object%20Reference) (OtherActor :type Actor%20Object%20Reference) (OtherComp :type Primitive%20Component%20Object%20Reference) (OtherBodyIndex :type Integer) (bFromSweep :type Boolean) (SweepResult :type Hit%20Result%20Structure%20%28by%20ref%29))
  ;[1 1 1] BeginOverlap
  (bind _asentity_master_bp (Utilities|Casting|CastToentityMasterBp OtherActor))
  (Utilities|FlowControl|Sequence
    (:then_0
      (for _array_element (Variables|/Script/Engine.ActorComponent|GetComponentTags (Variables|/Game/Blueprints/Resources/entityMasterBp.entityMasterBp_C|GetBox _asentity_master_bp))
        (if (Utilities|Name|Equal(Name) _array_element "obstacle")
          (Variables|Default|SetmoveSpeed 0.0))))
    (:then_1
      (for _array_element_2 (Variables|/Script/Engine.ActorComponent|GetComponentTags (Variables|/Game/Blueprints/Resources/entityMasterBp.entityMasterBp_C|GetBox _asentity_master_bp))
        (if (Utilities|Name|Equal(Name) _array_element_2 "enmHit")
          (if (Utilities|IsValid _asentity_master_bp) :!label _label
            (Variables|Default|Sethit? true)
            (Default|EntityDmg _asentity_master_bp (Utilities|Struct|BreakenemyStatsStr (Variables|Default|GetStats)) (.Health (Utilities|Struct|BreakentityStats (Variables|/Game/Blueprints/Resources/entityMasterBp.entityMasterBp_C|GetentStats _asentity_master_bp))))
            (Utilities|FlowControl|Delay (Utilities|Struct|BreakenemyStatsStr (Variables|Default|GetStats)))
            (goto _label)))))
    (:then_2
      (for _array_element_3 (Variables|/Script/Engine.ActorComponent|GetComponentTags (Variables|/Game/Blueprints/Resources/entityMasterBp.entityMasterBp_C|GetBox _asentity_master_bp))
        (if (Utilities|Name|Equal(Name) _array_element_3 "trapDmg")
          (if (Utilities|IsValid _asentity_master_bp)
            (CallFunction|EntityDmg (Math|Conversions|ToFloat(Integer) (Utilities|Struct|BreakentityStats (Variables|/Game/Blueprints/Resources/entityMasterBp.entityMasterBp_C|GetentStats _asentity_master_bp))) (Utilities|Struct|BreakenemyStatsStr (Variables|Default|GetStats)))
            (Utilities|FlowControl|Delay 0.5)
            (Actor|DestroyActor _asentity_master_bp)))))))

(event OnComponentEndOverlap(Box)
  (params (OverlappedComponent :type Primitive%20Component%20Object%20Reference) (OtherActor :type Actor%20Object%20Reference) (OtherComp :type Primitive%20Component%20Object%20Reference) (OtherBodyIndex :type Integer))
  ;[1 1 1] EndOverlap
  (bind _asentity_master_bp (Utilities|Casting|CastToentityMasterBp OtherActor))
  (for _array_element (Variables|/Script/Engine.ActorComponent|GetComponentTags (Variables|/Game/Blueprints/Resources/entityMasterBp.entityMasterBp_C|GetBox _asentity_master_bp))
    (if (Utilities|Name|Equal(Name) _array_element "obstacle")
      (Variables|Default|Sethit? false)
      (Utilities|FlowControl|Delay 2.0)
      (Variables|Default|SetmoveSpeed (.Speed (Utilities|Struct|BreakenemyStatsStr (Variables|Default|GetStats)))))))

(event EventBeginPlay
  ;[1 1 1] BeginPlay
  (|CallParentFunction)
  (CallFunction|GetRandomMaterial "/Game/Zombie/Zombie_01/Materials/M_Zombie01_02.M_Zombie01_02" "/Game/Zombie/Zombie_01/Materials/M_Zombie01_01.M_Zombie01_01" "/Game/Zombie/Zombie_01/Materials/M_Zombie01_03.M_Zombie01_03" "/Game/Zombie/Zombie_01/Materials/M_Zombie01_04.M_Zombie01_04")
  (bind _returnvalue (Actor|GetActorOfClass "/Game/meleeActor.meleeActor_C"))
  (Variables|Default|SetmeleeBp _returnvalue)
  (bind _returnvalue_2 (Actor|GetActorOfClass "/Game/rangeActor.rangeActor_C"))
  (Variables|Default|SetrangeBp _returnvalue_2)
  (Variables|Default|SetmoveSpeed (.Speed (Utilities|Struct|BreakenemyStatsStr (Variables|Default|GetStats))))
  (bind _asfp_splayer_controller (Utilities|Casting|CastToFpSPlayerController (Game|GetPlayerController 0)))
  (Variables|Default|SetplContr _asfp_splayer_controller)
  (bind _returnvalue_3 (Actor|GetActorOfClass "/Game/Blueprints/DebugModeBp.DebugModeBp_C"))
  (Variables|Default|SetdebugMode _returnvalue_3))

(event Collision|EventActorBeginOverlap
  (params (OtherActor :type Actor%20Object%20Reference))
  (|CallParentFunction OtherActor) ; This node is disabled and will not be called.\nDrag off pins to build functionality.
)

(event EventTick
  (params (DeltaSeconds :type Float%20%28single-precision%29))
  (bind _self self)
  ;[1 1 1] Tick
  (|CallParentFunction DeltaSeconds)
  (if (Utilities|IsValid _self)
    (Class|Actor|AddActorLocalTransform (Math|Transform|MakeTransform (Math|Vector|MakeVector (Variables|Default|GetmoveSpeed) 0.0 0.0) "0, 0, 0" "1,1,1") false false)
    (if (< (.x (Transformation|GetActorLocation _self)) -3.7e+02)
      (Utilities|FlowControl|DoOnce false
        (:Completed
          (bind _asfp_splayer_controller (Utilities|Casting|CastToFpSPlayerController (Game|GetPlayerController 0)))
          (Variables|/Game/Blueprints/FpSPlayerController.FpSPlayerController_C|Sethealth _asfp_splayer_controller (- (Variables|/Game/Blueprints/FpSPlayerController.FpSPlayerController_C|Gethealth _asfp_splayer_controller) (Utilities|Struct|BreakenemyStatsStr (Variables|Default|GetStats))))
          (Actor|DestroyActor))))))

(fn ConstructionScript
  (|CallParentFunction))

(fn GetItemDistance
  (bind _self self)
  (bind _skeletalmesh (Variables|Default|GetSkeletalMesh _self))
  (bind _returnvalue (Transformation|GetWorldLocation _skeletalmesh))
  (if (<= (.x _returnvalue) (.x (Transformation|GetWorldLocation (Variables|/Game/meleeActor.meleeActor_C|GetDefaultSceneRoot (Variables|Default|GetmeleeBp)))))
    (bind _item (Default|GetEquipedItem (Variables|Default|GetInvSysBp) "NewEnumerator6"))
    (if (Utilities|Enum|Equal(Enum) (Utilities|Struct|BreaktoolsStr (Variables|/Game/Blueprints/Tools/ToolsMaster.ToolsMaster_C|Getinfo _item)) "NewEnumerator2")
      (LocalVariables|Setweapon _item)
      (LocalVariables|Sethit true)
      (Variables|Default|Setrange? false)
      (else
        (LocalVariables|Sethit false)))
    (return (LocalVariables|Getweapon) (LocalVariables|Gethit))
    (elif (<= (.x _returnvalue) (.x (Transformation|GetWorldLocation (Variables|/Game/rangeActor.rangeActor_C|GetDefaultSceneRoot (Variables|Default|GetrangeBp)))))
      (bind _item_2 (Default|GetEquipedItem (Variables|Default|GetInvSysBp) "NewEnumerator6"))
      (if (Utilities|Enum|Equal(Enum) (.type (Variables|/Game/Blueprints/Tools/ToolsMaster.ToolsMaster_C|Getinfo _item_2)) "NewEnumerator3")
        (LocalVariables|Setweapon _item_2)
        (LocalVariables|Sethit true)
        (Variables|Default|Setrange? true)
        (else
          (Development|PrintString "Cant Reach")
          (LocalVariables|Sethit false)
          (Variables|Default|Setrange? false)))
      (return (LocalVariables|Getweapon) (LocalVariables|Gethit)))))

(fn GetRandomMaterial
  (params (Material_01 :type Material%20Object%20Reference) (Material_02 :type Material%20Object%20Reference) (Material_03 :type Material%20Object%20Reference) (Material_04 :type Material%20Object%20Reference))
  (switch int (Math|Random|RandomIntegerinRange 0 3)
    (:0
      (Rendering|Material|SetMaterial (Variables|Default|GetSkeletalMesh) 0 Material_01))
    (:1
      (Rendering|Material|SetMaterial (Variables|Default|GetSkeletalMesh) 0 Material_02))
    (:2
      (Rendering|Material|SetMaterial (Variables|Default|GetSkeletalMesh) 0 Material_03))
    (:3
      (Rendering|Material|SetMaterial (Variables|Default|GetSkeletalMesh) 0 Material_04))))

(fn CheckAmmunition
  (params (Selection :type Integer))
  (bind _plcontr (Variables|Default|GetplContr))
  (switch int Selection
    (:1
      (if (> (Variables|/Game/Blueprints/FpSPlayerController.FpSPlayerController_C|Getstone _plcontr) 0)
        (Variables|/Game/Blueprints/FpSPlayerController.FpSPlayerController_C|Setstone _plcontr (- (Variables|/Game/Blueprints/FpSPlayerController.FpSPlayerController_C|Getstone _plcontr) 1))
        (LocalVariables|Sethas? true)
        (else
          (LocalVariables|Sethas? false))))
    (:2
      (if (and (> (Variables|/Game/Blueprints/FpSPlayerController.FpSPlayerController_C|Getwood _plcontr) 0) (> (Variables|/Game/Blueprints/FpSPlayerController.FpSPlayerController_C|Getiron _plcontr) 0))
        (Variables|/Game/Blueprints/FpSPlayerController.FpSPlayerController_C|Setwood _plcontr (- (Variables|/Game/Blueprints/FpSPlayerController.FpSPlayerController_C|Getwood _plcontr) 1))
        (Variables|/Game/Blueprints/FpSPlayerController.FpSPlayerController_C|Setiron _plcontr (- (Variables|/Game/Blueprints/FpSPlayerController.FpSPlayerController_C|Getiron _plcontr) 1))
        (LocalVariables|Sethas? true)
        (else
          (LocalVariables|Sethas? false))))
    (:3
      (if (and (> (Variables|/Game/Blueprints/FpSPlayerController.FpSPlayerController_C|Getiron _plcontr) 0) (> (Variables|/Game/Blueprints/FpSPlayerController.FpSPlayerController_C|Getwood _plcontr) 0))
        (Variables|/Game/Blueprints/FpSPlayerController.FpSPlayerController_C|Setwood _plcontr (- (Variables|/Game/Blueprints/FpSPlayerController.FpSPlayerController_C|Getwood _plcontr) 1))
        (Variables|/Game/Blueprints/FpSPlayerController.FpSPlayerController_C|Setiron _plcontr (- (Variables|/Game/Blueprints/FpSPlayerController.FpSPlayerController_C|Getiron _plcontr) 1))
        (LocalVariables|Sethas? true)
        (else
          (LocalVariables|Sethas? false)))))
  (return (LocalVariables|Gethas?)))