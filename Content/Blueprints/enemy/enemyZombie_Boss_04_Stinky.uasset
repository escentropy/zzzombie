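; Stinky zombie boss that switches to its own soundtrack, advances along X and lobs a throwable that spawns a regular zombie.
; Tick halts it past an X threshold, then after a delay triggers the timeline-animated throw if no zombie occupies the landing point.
; Box overlaps stop it at obstacles or repeatedly damage tagged entities.
; Tick also destroys it on death, or damages the player if it moves past the far boundary.
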(event OnComponentBeginOverlap(Box)
  (params (OverlappedComponent :type Primitive%20Component%20Object%20Reference) (OtherActor :type Actor%20Object%20Reference) (OtherComp :type Primitive%20Component%20Object%20Reference) (OtherBodyIndex :type Integer) (bFromSweep :type Boolean) (SweepResult :type Hit%20Result%20Structure%20%28by%20ref%29))
  ;[1 1 1] overlap
  (bind _asentity_master_bp (Utilities|Casting|CastToentityMasterBp OtherActor))
  (Utilities|FlowControl|Sequence
    (:then_0
      (for _array_element (Variables|/Script/Engine.ActorComponent|GetComponentTags (Variables|/Game/Blueprints/Resources/entityMasterBp.entityMasterBp_C|GetBox _asentity_master_bp))
        (if (Utilities|Name|Equal(Name) _array_element "obstacle")
          (Variables|Default|SetmoveSpeed 0.0))))
    (:then_1
      (for _array_element_2 (Variables|/Script/Engine.ActorComponent|GetComponentTags (Variables|/Game/Blueprints/Resources/entityMasterBp.entityMasterBp_C|GetBox _asentity_master_bp))
        (if (Utilities|Name|Equal(Name) _array_element_2 "enmHit")
          (if (Utilities|IsValid _asentity_master_bp) :!label _label
            (Variables|Default|Sethit? true)
            (Variables|/Game/Blueprints/Resources/entityMasterBp.entityMasterBp_C|SetconstHealth _asentity_master_bp (- (Variables|/Game/Blueprints/Resources/entityMasterBp.entityMasterBp_C|GetconstHealth _asentity_master_bp) 25.0))
            (Utilities|FlowControl|Delay 2.0)
            (Utilities|FlowControl|Delay 1.0)
            (goto _label)))))))

(event Custom|ability
  (bind _throwable (Variables|Default|Getthrowable))
  ;[1 1 1] ability
  (Development|SetHiddeninGame _throwable false false)
  (bind (_direction _x _z) (Timeline|abilityTimeline PlayFromStart)
    (:Update
      (Transformation|AddRelativeLocation _throwable (Math|Vector|MakeVector _x 0.0 _z) false false))
    (:Finished
      (Variables|Default|SetmoveSpeed 0.0)
      (Development|SetHiddeninGame _throwable true false)
      (Transformation|SetRelativeLocation _throwable (Variables|Default|GetrockDefaultVector) false false)
      (Game|SpawnActorfromClass "/Game/Blueprints/enemy/enemyZombie.enemyZombie_C" (Math|Transform|MakeTransform (Transformation|GetWorldLocation (Variables|Default|GetendPpointVector)) "0, 0, 0" "1,1,1") "Undefined" 0 0))))

(event EventTick
  (params (DeltaSeconds :type Float%20%28single-precision%29))
  (bind _self self)
  ;[1 1 1] tick
  (if (Utilities|IsValid _self)
    (bind _isdead (CallFunction|ChkDead))
    (if _isdead
      (Utilities|FlowControl|Delay 2.0)
      (Actor|DestroyActor)
      (else
        (Utilities|FlowControl|Sequence
          (:then_0
            (if (== (Utilities|Array|Length (Collision|GetOverlappingActors (Variables|Default|GetendPoint) "/Game/Blueprints/enemy/enemyZombie.enemyZombie_C" :!class /Script/Engine.PrimitiveComponent)) 0)
              (Variables|Default|SetcanThrow true)
              (else
                (Variables|Default|SetcanThrow false))))
          (:then_1
            (if (< (.x (Transformation|GetWorldLocation (Variables|Default|GetBox))) 301.0)
              (Variables|Default|SetmoveSpeed 0.0)
              (Utilities|FlowControl|Delay 1e+01)
              (if (Variables|Default|GetcanThrow)
                (CallFunction|Ability))
              (else
                (Class|Actor|AddActorLocalTransform (Math|Transform|MakeTransform (Math|Vector|MakeVector (Variables|Default|GetmoveSpeed) 0.0 0.0) "0, 0, 0" "1,1,1") false false)
                (if (< (.x (Transformation|GetActorLocation _self)) -3.7e+02)
                  (Utilities|FlowControl|DoOnce false
                    (:Completed
                      (bind _asfp_splayer_controller (Utilities|Casting|CastToFpSPlayerController (Game|GetPlayerController 0)))
                      (Variables|/Game/Blueprints/FpSPlayerController.FpSPlayerController_C|Sethealth _asfp_splayer_controller (- (Variables|/Game/Blueprints/FpSPlayerController.FpSPlayerController_C|Gethealth _asfp_splayer_controller) (.AttackHero (Utilities|Struct|BreakenemyStatsStr (Variables|Default|GetStats)))))
                      (CallFunction|BossIsDead)
                      (Actor|DestroyActor))))))))))))

(event EventBeginPlay
  ;[1 1 1] BeginPlay
  (|CallParentFunction)
  (CallFunction|GetRandomMaterial)
  (Variables|Default|SetrockDefaultVector (Variables|/Script/Engine.SceneComponent|GetRelativeLocation (Variables|Default|Getthrowable)))
  (if (not (Variables|Default|Geteditor_0))
    (CallFunction|ChangeSoundtrack)
    (Variables|Default|SetIsBoss? true)))

(fn ConstructionScript
  (|CallParentFunction)
  (CallFunction|GetRandomMaterial)
  (Variables|Default|SetSpecialSoundtrack "/Game/Sounds/SoundtrackParts/part_3_boss_2__DnB__Cue.part_3_boss_2__DnB__Cue"))