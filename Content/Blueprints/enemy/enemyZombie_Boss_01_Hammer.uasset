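; Hammer-wielding zombie boss, a child enemy Blueprint that adds a weapon and boss soundtrack to inherited behavior.
; On BeginPlay it randomizes its material, attaches a spawned BossHammer_bp to a left-hand socket and, unless Editor0 is set, switches music and flags itself as boss.
; Tick polls IsDead, then calls BossIsDead and destroys the hammer, using the hammer's validity as a guard.
; The construction script assigns the boss's special soundtrack cue.
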(event EventBeginPlay
  (|CallParentFunction)
  (CallFunction|GetRandomMaterial)
  ;[1 1 1] Equip Weapon
  (bind _returnvalue (Game|SpawnActorfromClass "/Game/Zombie/Zombie_boss_02/Equipments/BossHammer_bp.BossHammer_bp_C" (Transformation|GetActorTransform) "Undefined" 0 0))
  (bind _output_get (Variables|Default|Sethammer _returnvalue))
  (Transformation|AttachComponentToComponent _output_get (Variables|Default|GetSkeletalMesh) "Bip001-L-Finger0Socket" "SnapToTarget" "SnapToTarget" "SnapToTarget" true)
  (if (not (Variables|Default|Geteditor_0))
    (CallFunction|ChangeSoundtrack)
    (Variables|Default|SetIsBoss? true)))

(event Collision|EventActorBeginOverlap
  (params (OtherActor :type Actor%20Object%20Reference))
  (|CallParentFunction OtherActor) ; This node is disabled and will not be called.\nDrag off pins to build functionality.
)

(event EventTick
  (params (DeltaSeconds :type Float%20%28single-precision%29))
  (bind _hammer (Variables|Default|Gethammer))
  (|CallParentFunction DeltaSeconds)
  (if (Variables|Default|GetisDead)
    (if (Utilities|IsValid _hammer)
      (CallFunction|BossIsDead)
      (Actor|DestroyActor _hammer))))

(fn ConstructionScript
  (|CallParentFunction)
  (Variables|Default|SetSpecialSoundtrack "/Game/Sounds/SoundtrackParts/Part_2_Boss_1___main_funk__Cue.Part_2_Boss_1___main_funk__Cue"))